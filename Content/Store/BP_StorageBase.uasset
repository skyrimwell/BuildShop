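; BP_StorageBase is a base storage slot that previews and accepts items placed into it.
; Its collision overlap sends the other actor a store preview message with whether the slot is free, saving the reply as the potential item.
; Ending the overlap stops that preview.
; Both add events pass the potential item, which AddItem first replaces with its argument, to an empty OnAddItem event.
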(event `self.SlotCollision.OnComponentBeginOverlap`
  (params (OverlappedComponent :type "PrimitiveComponent Object Reference") (OtherActor :type "Actor Object Reference") (OtherComp :type "PrimitiveComponent Object Reference") (OtherBodyIndex :type Integer) (bFromSweep :type Boolean) (SweepResult :type "HitResult Structure (by ref)"))
  (bind (_laststoreditemstack_item _laststoreditemstack_itemquantity) (break `/Game/GameManage/ST_ItemStack` (`self.LastStoredItemStack`)))
  (bind _newparam (message `/Game/BP_Main/BPI_Storable.Store Preview` OtherActor (== _laststoreditemstack_itemquantity 0) self))
  (set `self.Potential Item` _newparam))

(event `self.SlotCollision.OnComponentEndOverlap`
  (params (OverlappedComponent :type "PrimitiveComponent Object Reference") (OtherActor :type "Actor Object Reference") (OtherComp :type "PrimitiveComponent Object Reference") (OtherBodyIndex :type Integer))
  (message `/Game/BP_Main/BPI_Storable.StorePreviewStop` OtherActor))

(event `Add potential item`
  (`self.OnAddItem` (`self.Potential Item`) :!label _label))

(event `AddItem`
  (params (ItemToAdd :type "/Game/GameManage/ST_ItemStack Structure"))
  (set `self.Potential Item` ItemToAdd)
  (goto _label))

(event `OnAddItem`
  (params (Item :type "/Game/GameManage/ST_ItemStack Structure")))

(fn `UserConstructionScript`)