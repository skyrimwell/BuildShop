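; Draggable shop item actor that the player picks up with the mouse and drops into a storage slot.
; Clicking grabs the mesh with a PhysicsHandle, and Tick moves it to the cursor ray's intersection with a fixed-X depth plane.
; Slots trigger StorePreview to show a sprite icon; releasing there stores and destroys the item, otherwise it returns to ReturnPoint after a delay.
; BeginPlay initializes it from a hard-coded hammer row in DT_Items.
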(event `/Game/BP_Main/BPI_Clickable.OnObjectClicked`
  (bind _returnvalue (`GameplayStatics.GetPlayerController` 0))
  ;[1 1 1] Поворот иконки товара(для store preview)
  (`SceneComponent.K2_SetWorldRotation` (`self.PaperSprite`) (`self.K2_GetActorRotation` (`self.PC_Ref`)) false false)
  (set `self.PC_Ref` _returnvalue)
  (`PhysicsHandleComponent.GrabComponentAtLocation` (`self.PhysicsHandle`) (`self.SM`) "None" (`PrimitiveComponent.GetCenterOfMass` (`.HitComponent` (`GameplayStatics.BreakHitResult` (`PlayerController.GetHitResultUnderCursorByChannel` _returnvalue "TraceTypeQuery1" true))) "None"))
  (set `self.isDragging` true))

(event `self.ReceiveBeginPlay`
  (cast `/Game/BP_Main/BuildShopGameState` (`GameplayStatics.GetGameState`))
  (bind _returnvalue (`|GetDataTableRow` "/Game/GameManage/DT_Items.DT_Items" "I_Hammer")
    (:`then`
      (`StaticMeshComponent.SetStaticMesh` (`self.SM`) null)
      (set `self.ItemInfo` (make `/Game/GameManage/ST_ItemStack` (make `/Game/GameManage/ST_Item` "Ыщьу" 0 "/Game/Store/05267095756067_Y3JvcCw4MDgsNjMyLDAsMA.05267095756067_Y3JvcCw4MDgsNjMyLDAsMA" 0 0.0 "/Engine/BasicShapes/Cone.Cone")))
      (set `self.PC_Ref` (`GameplayStatics.GetPlayerController` 0)))))

(event `self.ReceiveTick`
  (params (DeltaSeconds :type "Float (single-precision)"))
  (bind _pc_ref (`self.PC_Ref`))
  (bind (_locationx _locationy) (`PlayerController.GetMousePosition` _pc_ref))
  (bind (_worldposition _worlddirection) (`GameplayStatics.DeprojectScreenToWorld` _pc_ref (`KismetMathLibrary.MakeVector2D` _locationx _locationy)))
  (if (`self.isDragging`)
    (`PhysicsHandleComponent.SetTargetLocation` (`self.PhysicsHandle`) (+ _worldposition (* _worlddirection (`KismetMathLibrary.SafeDivide` (- (`self.BaseDepthX`) (.x _worldposition)) (.x _worlddirection)))))
    ;[1 1 1] Выход из стейта захвата
    (if (not (`PlayerController.IsInputKeyDown` (`self.PC_Ref`) "LeftMouseButton"))
      (`PhysicsHandleComponent.ReleaseComponent` (`self.PhysicsHandle`))
      (set `self.isDragging` false)
      (if (`self.TargetBoxSelected`)
        (`/Game/BP_Main/BPI_Storable.Store`)
        (else
          ;[1 1 1] Гашение инерции
          (`PhysicsHandleComponent.SetTargetLocation` (`self.PhysicsHandle`) (`SceneComponent.RelativeLocation` (`self.SM`)))
          (`KismetSystemLibrary.Delay` 0.5)
          (`self.ReturnToPoint`))))))

(event `/Game/BP_Main/BPI_Storable.StorePreviewStop`
  (`SceneComponent.SetVisibility` (`self.PaperSprite`) false false)
  (`SceneComponent.SetVisibility` (`self.SM`) true false)
  (set `self.TargetBoxSelected` false))

(event `/Game/BP_Main/BPI_Storable.Store`
  (bind _sm (`self.SM`))
  (`/Game/Store/BP_StorageSlot.Add potential item` (`self.SlotRef`))
  (`PrimitiveComponent.SetEnableGravity` _sm false)
  (`PrimitiveComponent.SetSimulatePhysics` _sm false)
  (`/Engine/EditorBlueprintResources/StandardMacros.IsValid` self
    (:`Is Valid`
      (`self.K2_DestroyActor` self))))

(fn `ReturnToPoint`
  (bind _returnpoint (`self.ReturnPoint`))
  (bind _sm (`self.SM`))
  (`/Engine/EditorBlueprintResources/StandardMacros.IsValid` _returnpoint
    (:`Is Valid`
      (`KismetSystemLibrary.PrintString` "ValidPoint")
      (`PrimitiveComponent.SetSimulatePhysics` _sm true)
      (`SceneComponent.K2_SetRelativeLocation` _sm (`self.K2_GetActorLocation` _returnpoint) false false))
    (:`Is Not Valid`
      (`KismetSystemLibrary.PrintString` "PointIsNotValid"))))

(fn `Store Preview`
  (params (IsFree :type Boolean) (StorageSlot :type "/Game/Store/BP_StorageSlot Object Reference"))
  (returns (NewParam :type "/Game/GameManage/ST_ItemStack Structure"))
  (set `self.SlotRef` StorageSlot)
  (`SceneComponent.SetVisibility` (`self.PaperSprite`) true false)
  (`SceneComponent.SetVisibility` (`self.SM`) (not IsFree) false)
  (set `self.TargetBoxSelected` true)
  (return (`self.ItemInfo`)))

(fn `UserConstructionScript`)