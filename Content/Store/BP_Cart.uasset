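; BP_Cart is a store shopping cart actor that holds item stacks in a CartStorage map keyed by ItemID.
; OnAddItem merges quantities into an existing stack or inserts a new one, and ClearCart empties the map.
; ShowCart prints each item's name and quantity as debug output, and runs only after a new item is inserted.
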(event `ClearCart`
  (`BlueprintMapLibrary.Map_Clear` (`self.CartStorage`)))

(event `self.OnAddItem`
  (params (Item :type "/Game/GameManage/ST_ItemStack Structure"))
  (bind (_item _itemquantity) (break `/Game/GameManage/ST_ItemStack` Item))
  (bind (_item_2 _itemquantity_2) (break `/Game/GameManage/ST_ItemStack` Item))
  (bind (_value _returnvalue) (`BlueprintMapLibrary.Map_Find` (`self.CartStorage`) (`.ItemID_10_05E1392B4735FFE91395E096C0362B11` (break `/Game/GameManage/ST_Item` _item))))
  (bind (_item_3 _itemquantity_3) (break `/Game/GameManage/ST_ItemStack` _value))
  (if _returnvalue
    (`BlueprintMapLibrary.Map_Add` (`self.CartStorage`) (`.ItemID_10_05E1392B4735FFE91395E096C0362B11` (break `/Game/GameManage/ST_Item` _item_3)) (make `/Game/GameManage/ST_ItemStack` _item_3 (+ _itemquantity_3 _itemquantity)))
    (else
      (`BlueprintMapLibrary.Map_Add` (`self.CartStorage`) (`.ItemID_10_05E1392B4735FFE91395E096C0362B11` (break `/Game/GameManage/ST_Item` _item_2)) Item)
      (`KismetSystemLibrary.PrintString` (`KismetStringLibrary.Concat_StrStr` "Add new item: \n" (`KismetStringLibrary.Conv_NameToString` (break `/Game/GameManage/ST_Item` _item_2)) " \n" (`KismetStringLibrary.Conv_IntToString` _itemquantity_2)))
      (`self.ShowCart`))))

(event `ShowCart`
  (bind _cartstorage (`self.CartStorage`))
  (bind _keys (`BlueprintMapLibrary.Map_Keys` _cartstorage))
  (for _array_element _keys
    (bind _value (`BlueprintMapLibrary.Map_Find` _cartstorage _array_element))
    (`KismetSystemLibrary.PrintString` (`KismetStringLibrary.Concat_StrStr` "___________ \n" (`KismetStringLibrary.Conv_NameToString` (break `/Game/GameManage/ST_Item` (break `/Game/GameManage/ST_ItemStack` _value))) " \nКоличество:" (`KismetStringLibrary.Conv_IntToString` (`.ItemQuantity_4_F5DAE9484DE62FBE49B5F0A69999838A` (break `/Game/GameManage/ST_ItemStack` _value))) "-------------- \n"))))

(fn `UserConstructionScript`
  (`parent.UserConstructionScript`))