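; BP_StoredItemOld is a store item actor that the player drags with the mouse as a physics object.
; Clicking it grabs the mesh through a PhysicsHandle at the center of mass of the component under the cursor.
; While dragging, Tick deprojects the cursor onto a fixed world-Y plane at BaseDepthY and sets the handle target there.
; Releasing the left mouse button drops it and resets the target to the mesh's relative location, intended to damp inertia.
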(event `/Game/BP_Main/BPI_Clickable.OnObjectClicked`
  (bind _returnvalue (`GameplayStatics.GetPlayerController` 0))
  (set `self.PC_Ref` _returnvalue)
  (`PhysicsHandleComponent.GrabComponentAtLocation` (`self.PhysicsHandle`) (`self.SM`) "None" (`PrimitiveComponent.GetCenterOfMass` (`.HitComponent` (`GameplayStatics.BreakHitResult` (`PlayerController.GetHitResultUnderCursorByChannel` _returnvalue "TraceTypeQuery1" true))) "None"))
  (set `self.isDragging` true))

(event `CustomEvent`)

(event `self.ReceiveTick`
  (params (DeltaSeconds :type "Float (single-precision)"))
  (bind _pc_ref (`self.PC_Ref`))
  (bind (_locationx _locationy) (`PlayerController.GetMousePosition` _pc_ref))
  (bind (_worldposition _worlddirection) (`GameplayStatics.DeprojectScreenToWorld` _pc_ref (`KismetMathLibrary.MakeVector2D` _locationx _locationy)))
  (if (`self.isDragging`)
    (`PhysicsHandleComponent.SetTargetLocation` (`self.PhysicsHandle`) (+ _worldposition (* _worlddirection (`KismetMathLibrary.SafeDivide` (- (`self.BaseDepthY`) (.y _worldposition)) (.y _worlddirection)))))
    ;[1 1 1] Выход из стейта захвата
    (if (not (`PlayerController.IsInputKeyDown` (`self.PC_Ref`) "LeftMouseButton"))
      (`PhysicsHandleComponent.ReleaseComponent` (`self.PhysicsHandle`))
      (set `self.isDragging` false)
      ;[1 1 1] Гашение инерции
      (`PhysicsHandleComponent.SetTargetLocation` (`self.PhysicsHandle`) (`SceneComponent.RelativeLocation` (`self.SM`)))
      (`KismetSystemLibrary.Delay` 0.5))))

(fn `UserConstructionScript`)