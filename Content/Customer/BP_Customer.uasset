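; BP_Customer is a customer actor that moves along a referenced spline between its points, starting at the beginning.
; Move-to, next and previous point events set a target distance, which Tick approaches at Speed, aligning the actor to the spline with a yaw offset.
; Stepping back plays a timeline turn before reversing.
; When the backward target is reached, Tick restores forward mode and turns the customer around again.
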(event `self.ReceiveBeginPlay`
  (bind _returnvalue (`self.GetComponentByClass` (`self.Spline`) "/Script/Engine.SplineComponent"))
  (bind (_returnvalue_location _returnvalue_rotation) (`KismetMathLibrary.BreakTransform` (`SplineComponent.GetTransformAtDistanceAlongSpline` _returnvalue 0.0 "World" false)))
  (set `self.SplineInfo` _returnvalue)
  (set `self.MaxPositionNum` (`SplineComponent.GetNumberOfSplinePoints` _returnvalue))
  (set `self.CurrentDistance` 0.0)
  (`self.K2_SetActorTransform` (`KismetMathLibrary.MakeTransform` _returnvalue_location (`KismetMathLibrary.MakeRotator` (.roll _returnvalue_rotation) (.pitch _returnvalue_rotation) (+ (.yaw _returnvalue_rotation) -90.0)))))

(event `self.ReceiveTick`
  (params (DeltaSeconds :type "Float (single-precision)"))
  (bind _returnvalue (- (`self.CurrentDistance`) (* DeltaSeconds (`self.Speed`))))
  (bind _returnvalue_2 (+ (* DeltaSeconds (`self.Speed`)) (`self.CurrentDistance`)))
  (bind (_returnvalue_location _returnvalue_rotation) (`KismetMathLibrary.BreakTransform` (`SplineComponent.GetTransformAtDistanceAlongSpline` (`self.SplineInfo`) _returnvalue_2 "World" false)))
  (bind (_returnvalue_location_2 _returnvalue_rotation_2) (`KismetMathLibrary.BreakTransform` (`SplineComponent.GetTransformAtDistanceAlongSpline` (`self.SplineInfo`) _returnvalue "World" false)))
  (if (`self.MoveForward`)
    ;[1 1 1] Движение вперед
    (if (<= _returnvalue_2 (`self.TargetDistance`))
      (`self.K2_SetActorTransform` (`KismetMathLibrary.MakeTransform` _returnvalue_location (`KismetMathLibrary.MakeRotator` (.roll _returnvalue_rotation) (.pitch _returnvalue_rotation) (+ (.yaw _returnvalue_rotation) -90.0))))
      (set `self.CurrentDistance` _returnvalue_2))
    (else
      ;[1 1 1] Движение назад
      (if (>= _returnvalue (`self.TargetDistance`))
        (`self.K2_SetActorTransform` (`KismetMathLibrary.MakeTransform` _returnvalue_location_2 (`KismetMathLibrary.MakeRotator` (.roll _returnvalue_rotation_2) (.pitch _returnvalue_rotation_2) (+ (.yaw _returnvalue_rotation_2) 90.0))))
        (set `self.CurrentDistance` _returnvalue)
        (else
          (set `self.MoveForward` true)
          (`self.RotateAround` true))))))

(event `MoveToSplinePoint`
  (params (PointNum :type Integer))
  (bind _output_get (set `self.CurrentPosition` PointNum))
  (set `self.TargetDistance` (`SplineComponent.GetDistanceAlongSplineAtSplinePoint` (`self.SplineInfo`) _output_get))
  (if (`self.MoveForward`)
    (set `self.MoveForward` true)))

(event `SetNextTargetPosition`
  (bind _result (`/Engine/EditorBlueprintResources/StandardMacros.IncrementInt` (`self.CurrentPosition`))
    (:`  `
      (set `self.TargetDistance` (`SplineComponent.GetDistanceAlongSplineAtSplinePoint` (`self.SplineInfo`) _result))
      (if (`self.MoveForward`)
        (set `self.MoveForward` true)))))

(event `SetPreviousTargetPosition`
  (bind _result (`/Engine/EditorBlueprintResources/StandardMacros.DecrementInt` (`self.CurrentPosition`))
    (:`  `
      (set `self.TargetDistance` (`SplineComponent.GetDistanceAlongSplineAtSplinePoint` (`self.SplineInfo`) _result))
      (if (`self.MoveForward`)
        (`self.RotateAround` false)
        (`KismetSystemLibrary.Delay` (`TimelineComponent.GetTimelineLength` (`self.RotationTimeLine`)))
        (set `self.MoveForward` false)))))

(event `RotateAround`
  (params (RotateInvert :type Boolean))
  (bind (_returnvalue_location _returnvalue_rotation) (`KismetMathLibrary.BreakTransform` (`SplineComponent.GetTransformAtDistanceAlongSpline` (`self.SplineInfo`) (`self.CurrentDistance`) "World" false)))
  (bind (_returnvalue_location_2 _returnvalue_rotation_2) (`KismetMathLibrary.BreakTransform` (`SplineComponent.GetTransformAtDistanceAlongSpline` (`self.SplineInfo`) (`self.CurrentDistance`) "World" false)))
  (set `self.StartRotation` (`self.K2_GetActorRotation`))
  (bind (_direction _rotationtrack) (`Timeline|RotationTimeLine` :!via `PlayFromStart`)
    (:`Update`
      (if RotateInvert
        (`self.K2_SetActorRotation` (`KismetMathLibrary.RLerp` (`self.StartRotation`) (`KismetMathLibrary.MakeRotator` (.roll _returnvalue_rotation) (.pitch _returnvalue_rotation) (- (.yaw _returnvalue_rotation) 90.0)) _rotationtrack true))
        (else
          (`self.K2_SetActorRotation` (`KismetMathLibrary.RLerp` (`self.StartRotation`) (`KismetMathLibrary.MakeRotator` (.roll _returnvalue_rotation_2) (.pitch _returnvalue_rotation_2) (+ (.yaw _returnvalue_rotation_2) 90.0)) _rotationtrack true)))))
    (:`Finished`
      (`KismetSystemLibrary.PrintString` "Finish timeline"))))

(fn `UserConstructionScript`)