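; Shop map scene controller that switches the time of day by rotating the main directional light.
; On BeginPlay it finds the light component tagged MainDirectionalLight, stores preset sun rotations and starts in evening.
; ManualAdvanceTime uses a counter to cycle evening, morning and midday, printing each state name.
; The night state exists but reuses the evening rotation and is not part of the cycle.
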(event `self.ReceiveBeginPlay`
  (bind _outactors (`GameplayStatics.GetAllActorsOfClass` "/Script/Engine.DirectionalLight"))
  (for _array_element _outactors
    _)
  (if (`self.ComponentHasTag` (`Light.LightComponent` _array_element) "MainDirectionalLight")
    (set `self.SunObject` (`Actor.FindComponentByTag` _array_element "/Script/Engine.DirectionalLightComponent" "MainDirectionalLight"))
    (set `self.MorningSunTransform` (struct :`Pitch` -163.0 :`Yaw` -309.0))
    (set `self.MiddaySunTransform` (struct :`Pitch` -140.0 :`Yaw` -261.0))
    (set `self.EveningSunTransform` (struct :`Pitch` -170.0 :`Yaw` 129.0))
    (`self.SetEveningState`)
    (else
      (`KismetSystemLibrary.PrintString` "No One Directional light"))))

(event `SetMorningState`
  (`self.K2_SetRelativeRotation` (`self.SunObject`) (`self.MorningSunTransform`) false false)
  (`KismetSystemLibrary.PrintText` "Rotation has been chamged"))

(event `SetMiddayState`
  (`self.K2_SetRelativeRotation` (`self.SunObject`) (`self.MiddaySunTransform`) false false))

(event `ManualAdvanceTime`
  (switch `int` (`self.counter`)
    (:`0`
      (bind _result (`/Engine/EditorBlueprintResources/StandardMacros.IncrementInt` (`self.counter`))
        (:`  `
          (set `self.counter` _result)
          (`self.SetEveningState`)
          (`KismetSystemLibrary.PrintString` "Evening"))))
    (:`1`
      (bind _result_2 (`/Engine/EditorBlueprintResources/StandardMacros.IncrementInt` (`self.counter`))
        (:`  `
          (set `self.counter` _result_2)
          (`self.SetMorningState`)
          (`KismetSystemLibrary.PrintString` "Morning"))))
    (:`2`
      (bind _result_3 (`/Engine/EditorBlueprintResources/StandardMacros.IncrementInt` (`self.counter`))
        (:`  `
          (set `self.counter` _result_3)
          (`self.SetMiddayState`)
          (`KismetSystemLibrary.PrintString` "Midday")
          (set `self.counter` 0))))))

(event `SetEveningState`
  (`self.K2_SetRelativeRotation` (`self.SunObject`) (`self.EveningSunTransform`) false false))

(event `SetNightState`
  (`self.K2_SetRelativeRotation` (`self.SunObject`) (`self.EveningSunTransform`) false false))