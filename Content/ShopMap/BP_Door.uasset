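; BP_Door is a clickable door in the shop map that switches the player between the storage and another shop position.
; On BeginPlay it caches the player's BP_ShopPawn and a BP_Cart actor, though the cart reference is not used afterwards.
; Clicking its Box component checks the pawn's AtTheStorage flag and calls MoveToCass if set, otherwise MoveToStore.
; The door mesh's click event is empty.
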(event `self.ReceiveBeginPlay`
  (bind _asbp_shop_pawn (cast `/Game/BP_Main/BP_ShopPawn` (`GameplayStatics.GetPlayerPawn` 0)))
  (set `self.PlayerRef` _asbp_shop_pawn)
  (bind _returnvalue (`GameplayStatics.GetActorOfClass` "/Game/Storage/BP_Cart.BP_Cart_C"))
  (set `self.CartRef` _returnvalue))

(event `self.Box.OnClicked`
  (params (TouchedComponent :type "PrimitiveComponent Object Reference") (ButtonPressed :type "Key Structure"))
  (bind _playerref (`self.PlayerRef`))
  (if (`/Game/BP_Main/BP_ShopPawn.AtTheStorage` (`self.PlayerRef`))
    (`/Game/BP_Main/BP_ShopPawn.MoveToCass` _playerref)
    (else
      (`/Game/BP_Main/BP_ShopPawn.MoveToStore` _playerref))))

(event `self.SM_Door.OnClicked`
  (params (TouchedComponent :type "PrimitiveComponent Object Reference") (ButtonPressed :type "Key Structure")))

(fn `UserConstructionScript`)