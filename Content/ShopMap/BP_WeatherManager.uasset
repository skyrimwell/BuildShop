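; Weather manager for the shop map that switches time of day between morning, midday, evening and night by rotating the sun.
; On BeginPlay it finds the sun and moon directional lights by component tag, then starts at morning.
; Each time-of-day event sets a target rotation that a timeline lerps toward, with the moon hidden for morning and revealed shortly after night starts.
; ManualAdvanceTime only increments a counter; its debug prints and reset are disconnected.
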(event `self.ReceiveBeginPlay`
  (bind _outactors (`GameplayStatics.GetAllActorsOfClass` "/Script/Engine.DirectionalLight"))
  (for _array_element _outactors
    (bind _lightcomponent (`Light.LightComponent` _array_element))
    (if (`ActorComponent.ComponentHasTag` _lightcomponent "MainDirectionalLight")
      (bind _returnvalue (`self.GetComponentByClass` _array_element "/Script/Engine.DirectionalLightComponent"))
      (set `self.Sun Object` _returnvalue)
      (elif (`ActorComponent.ComponentHasTag` _lightcomponent "Moon")
        (set `self.Moon` _returnvalue)
        (else
          (`KismetSystemLibrary.PrintString` "No One Directional light")))))
  (set `self.MorningSunTransform` (struct :`Pitch` -163.0 :`Yaw` -309.0))
  (set `self.MiddaySunTransform` (struct :`Pitch` -140.0 :`Yaw` -261.0))
  (set `self.EveningSunTransform` (struct :`Pitch` -170.0 :`Yaw` 129.0))
  (set `self.NightSunRotation` (struct :`Pitch` -181.0 :`Yaw` -204.0))
  (`self.SetMorning`))

(event `SetMorning`
  (`SceneComponent.SetHiddenInGame` (`self.Sun Object`) false true)
  (`SceneComponent.SetHiddenInGame` (`self.Moon`) true true)
  (set `self.TargetRotation` (`self.MorningSunTransform`))
  (`self.ChangeDayetimeTo`))

(event `SetMidday`
  (set `self.TargetRotation` (`self.MiddaySunTransform`))
  (`self.ChangeDayetimeTo`))

(event `ManualAdvanceTime`
  (switch `int` (`self.counter`)
    (:`0`
      (bind _result (`/Engine/EditorBlueprintResources/StandardMacros.IncrementInt` (`self.counter`))
        (:`  `
          (set `self.counter` _result))))
    (:`1`
      (bind _result_2 (`/Engine/EditorBlueprintResources/StandardMacros.IncrementInt` (`self.counter`))
        (:`  `
          (set `self.counter` _result_2))))
    (:`2`
      (bind _result_3 (`/Engine/EditorBlueprintResources/StandardMacros.IncrementInt` (`self.counter`))
        (:`  `
          (set `self.counter` _result_3))))
    (:`3`
      (bind _result_4 (`/Engine/EditorBlueprintResources/StandardMacros.IncrementInt` (`self.counter`))
        (:`  `
          (set `self.counter` _result_4))))))

(event `SetEvening`
  (set `self.TargetRotation` (`self.EveningSunTransform`))
  (`self.ChangeDayetimeTo`))

(event `Set night`
  (set `self.TargetRotation` (`self.NightSunRotation`))
  (`self.ChangeDayetimeTo`)
  (`KismetSystemLibrary.Delay` 0.5)
  (`SceneComponent.SetHiddenInGame` (`self.Moon`) false true))

(event `ChangeDayetimeTo`
  (bind _sun_object (`self.Sun Object`))
  (bind (_direction _newtrack_0) (`Timeline|Timeline` :!via `PlayFromStart`)
    (:`Update`
      (`SceneComponent.K2_SetRelativeRotation` _sun_object (`KismetMathLibrary.RLerp` (`SceneComponent.RelativeRotation` _sun_object) (`self.TargetRotation`) _newtrack_0 true) false false))))

(fn `UserConstructionScript`)