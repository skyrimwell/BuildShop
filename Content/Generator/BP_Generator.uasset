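; Customer order generator for a shop game that rolls each day's visitor and item counts, then builds an order per customer.
; GenerateOrder splits the customer's item share into entries and picks themed, incomplete, enum or math generators by entry size and probability.
; Generators draw DataTable rows affordable within the remaining budget per customer, mixing seeded and unseeded randomness.
; LineFormatter separately assembles dialogue text from theme descriptions or masked templates with declined item names.
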(event `self.ReceiveBeginPlay`)

(event `NextPeople`)

(fn `EnumGenerator`
  (params (ItemsCount :type Integer))
  (returns (GeneratedOrder :type "/Game/GameManage/ST_CustomerOrder Structure"))
  (bind _newparam (`self.GetAccessableSoloItems` ItemsCount))
  (bind _outitem (`KismetArrayLibrary.Array_Random` _newparam))
  (`|GetDataTableRow` "/Game/GameManage/DT_Items.DT_Items" _outitem
    (:`then`
      ; Change string
      (`KismetArrayLibrary.Array_Add` (`.Items_24_92E324BF40B28E2E42823A94930C01BA` (break `/Game/GameManage/ST_CustomerOrder` (`self.GeneratedOrder`))) (make `/Game/GameManage/ST_GroopedItems` "Enum elem" (`|MakeArray` (make `DataTableRowHandle` "/Game/GameManage/DT_Items.DT_Items" _outitem)) ItemsCount))
      (return))))

(fn `GenerateOrder`
  (returns (NewParam :type "/Game/GameManage/ST_CustomerOrder Structure"))
  (locals (CurrentClientItemsCount :type Integer) (ItemsForGen :type Integer))
  (bind _returnvalue (`KismetMathLibrary.RandomFloat`))
  (bind _itemsforgen (`local.ItemsForGen`))
  (bind (_generatedorder_customerline _generatedorder_items) (break `/Game/GameManage/ST_CustomerOrder` (`self.GeneratedOrder`)))
  (bind (_generatedorder_customerline_2 _generatedorder_items_2) (break `/Game/GameManage/ST_CustomerOrder` (`self.GeneratedOrder`)))
  (bind _returnvalue_2 (`KismetArrayLibrary.Array_Length` _generatedorder_items))
  (set `self.GeneratedOrder` (make `/Game/GameManage/ST_CustomerOrder` "Hi!"))
  (`/Engine/EditorBlueprintResources/StandardMacros.IncrementInt` (`self.CurrentClientNum`)
    (:`  `
      (if (!= (`self.CurrentClientNum`) (`self.CountOfPeople`))
        (bind _output_get (set `local.CurrentClientItemsCount` (`KismetMathLibrary.RandomIntegerInRangeFromStream` (`KismetMathLibrary.MakeRandomStream` (`self.Seed`)) 1 (- (`self.RemainingItems2`) (- (`self.CountOfPeople`) 1)))))
        (set `self.RemainingItems2` (- (`self.RemainingItems2`) _output_get))
        (else
          (set `local.CurrentClientItemsCount` (`self.RemainingItems2`))))
      ; Множественный заказ
      (while (!= (`local.CurrentClientItemsCount`) 0)
        (if (< _returnvalue_2 5)
          (bind _output_get_2 (set `local.ItemsForGen` (`KismetMathLibrary.RandomIntegerInRangeFromStream` (`KismetMathLibrary.MakeRandomStream` (`self.Seed`)) 1 (`local.CurrentClientItemsCount`))))
          (set `local.CurrentClientItemsCount` (- (`local.CurrentClientItemsCount`) _output_get_2))
          (else
            (`KismetSystemLibrary.PrintString` (`KismetStringLibrary.Conv_IntToString` _returnvalue_2) true true (struct :`G` 0.66 :`B` 1.0 :`A` 1.0) 20.0)
            (set `local.ItemsForGen` (`local.CurrentClientItemsCount`))
            (set `local.CurrentClientItemsCount` 0)))
        (if (== _output_get_2 1)
          (if (>= _returnvalue (`self.suggestionProbability`))
            (`self.SuggestionGenerator`)
            (elif (>= _returnvalue (`self.incompleteProbability`))
              (`self.IncompleteGenerator`)
              (else
                (`self.EnumGenerator` 1))))
          (elif (>= (`KismetMathLibrary.RandomFloat`) (`self.enum2Probability`))
            (`self.EnumGenerator` _itemsforgen)
            (else
              (`self.Math2Generator` _itemsforgen)))))
      (`KismetSystemLibrary.PrintString` (`KismetStringLibrary.Conv_IntToString` 0))
      (return (make `/Game/GameManage/ST_CustomerOrder` _generatedorder_customerline_2 _generatedorder_items_2)))))

(fn `GetAccessableGroupedItems`
  (params (Table :type "DataTable Object Reference") (Count :type Integer))
  (returns (NewParam :type "Array of Name"))
  (locals (AllNames :type "Array of Name") (ItemCount :type Integer) (SortedNames :type "Array of Name") (CurrentName :type Name))
  (set `local.ItemCount` Count)
  (bind _outrownames (`DataTableFunctionLibrary.GetDataTableRowNames` Table))
  (for _array_element _outrownames
    (set `local.CurrentName` _array_element)
    (bind _returnvalue (`|GetDataTableRow` Table _array_element)
      (:`then`
        (for _array_element_2 (`.ItemsRef_9_6F4167634A725D21C96609805CB749E4` (break `/Game/GameManage/ST_GroopedItems` _returnvalue))
          (bind (_datatable _rowname) (break `DataTableRowHandle` _array_element_2))
          (bind _returnvalue_2 (`|GetDataTableRow` _datatable _rowname)
            (:`then`
              (if (<= (* (`.ItemCost_20_EF3CC9BC4D8F1FE198FCE58B55A35F26` (break `/Game/GameManage/ST_Item` _returnvalue_2)) (`local.ItemCount`)) (/ (- (`self.averageDailyPrice`) (`self.completedPartOfPrice`)) (- (`self.CountOfPeople`) (`self.CurrentClientNum`))))
                (`KismetArrayLibrary.Array_Add` (`local.SortedNames`) (`local.CurrentName`))
                (break))))))))
  (return (`local.SortedNames`)))

(fn `GetAccessableSoloItems`
  (params (ItemsCount :type Integer))
  (returns (NewParam :type "Array of Name"))
  (locals (ItemCount :type Integer) (CurrentName :type Name) (SortedNames :type "Array of Name"))
  (set `local.ItemCount` ItemsCount)
  (bind _outrownames (`DataTableFunctionLibrary.GetDataTableRowNames` "/Game/GameManage/DT_Items.DT_Items"))
  (for _array_element _outrownames
    (set `local.CurrentName` _array_element)
    (bind _returnvalue (`|GetDataTableRow` "/Game/GameManage/DT_Items.DT_Items" _array_element)
      (:`then`
        (if (<= (* (`.ItemCost_20_EF3CC9BC4D8F1FE198FCE58B55A35F26` (break `/Game/GameManage/ST_Item` _returnvalue)) (`local.ItemCount`)) (/ (- (`self.averageDailyPrice`) (`self.completedPartOfPrice`)) (- (`self.CountOfPeople`) (`self.CurrentClientNum`))))
          (`KismetArrayLibrary.Array_Add` (`local.SortedNames`) (`local.CurrentName`))))))
  (return (`local.SortedNames`)))

(fn `IncompleteGenerator`
  (returns (GeneratedOrder :type "/Game/GameManage/ST_CustomerOrder Structure"))
  (locals (NewItem :type "/Game/GameManage/ST_GroopedItems Structure"))
  (bind _allthemeitems (`self.AllThemeItems`))
  (bind _generatedorder (`self.GeneratedOrder`))
  (bind _newitem_themedescription (break `/Game/GameManage/ST_GroopedItems` (`local.NewItem`)))
  (`KismetSystemLibrary.PrintString` "Incomplete gen")
  (bind _newparam (`self.GetAccessableGroupedItems` _allthemeitems 1))
  (bind _returnvalue (`|GetDataTableRow` _allthemeitems (`KismetArrayLibrary.Array_RandomFromStream` _newparam (`KismetMathLibrary.MakeRandomStream` (`KismetMathLibrary.RandomInteger` 10000))))
    (:`then`
      (bind (_themedescription _itemsref) (break `/Game/GameManage/ST_GroopedItems` _returnvalue))
      (bind _output_get (set `local.NewItem` (make `/Game/GameManage/ST_GroopedItems` _themedescription _itemsref 1)))
      (`KismetArrayLibrary.Array_Add` (`.Items_24_92E324BF40B28E2E42823A94930C01BA` (break `/Game/GameManage/ST_CustomerOrder` _generatedorder)) _output_get)
      (set `self.GeneratedOrder` _generatedorder)
      (set `self.CurrentOrderString` (`KismetStringLibrary.Concat_StrStr` (`self.CurrentOrderString`) _newitem_themedescription))
      (return))))

(fn `InitNewDay`
  (locals (WeightsSum :type "Float (double-precision)") (CurrentClientItemsCount :type Integer) (ItemsForGen :type Integer))
  (bind _seed (`self.Seed`))
  (bind _hellotablename (`self.HelloTableName`))
  (set `self.Seed` (`KismetMathLibrary.RandomInteger` 10000))
  (set `self.CurrentOrderString` (`KismetStringTableLibrary.GetTableEntrySourceString` _hellotablename (`KismetArrayLibrary.Array_Random` (`KismetStringTableLibrary.GetKeysFromStringTable` _hellotablename))))
  ; Генерация кол-ва покупателей и предметов
  (bind _output_get (set `self.CountOfPeople` (`KismetMathLibrary.RandomIntegerInRangeFromStream` (`KismetMathLibrary.MakeRandomStream` _seed) (`self.minPeople`) (`self.maxPeople`))))
  (bind _output_get_2 (set `self.dailyCountOfItems` (`KismetMathLibrary.RandomIntegerInRangeFromStream` (`KismetMathLibrary.MakeRandomStream` (`KismetMathLibrary.RandomIntegerFromStream` (`KismetMathLibrary.MakeRandomStream` _seed) 10000)) (`KismetMathLibrary.Max` (`self.minItems`) (`self.CountOfPeople`)) (`self.maxItems`))))
  (set `self.RemainingItems2` _output_get_2)
  (`KismetSystemLibrary.PrintString` (`KismetStringLibrary.Concat_StrStr` "Итого:" "Посетителей:" (`KismetStringLibrary.Conv_IntToString` _output_get) "Предметов:" (`KismetStringLibrary.Conv_IntToString` _output_get_2)) true true (struct :`G` 0.66 :`B` 1.0 :`A` 1.0) 20.0)
  (set `self.CurrentClientNum` 0))

(fn `LineFormatter`
  (params (CurrentOrderString :type String) (Stage :type "/Game/GameManage/DialogTables/E_OrderLineFormatter Enum" :default "NewEnumerator0") (Type :type "/Game/GameManage/DialogTables/E_OrderLineFormatterType Enum" :default "NewEnumerator5") (Thematic :type Name) (MathAmount :type Integer) (MathItem :type "/Game/GameManage/ST_Item Structure") (MathRowName :type Name))
  (returns (resultString :type String))
  (locals (currentAppendant :type Text))
  (bind _mathentrydialoguedt (`self.MathEntryDialogueDT`))
  (switch `/Game/GameManage/DialogTables/E_OrderLineFormatter` Stage
    (:`NewEnumerator0`
      ; Hello
      (switch `int` (`KismetMathLibrary.RandomIntegerInRangeFromStream` (`KismetMathLibrary.MakeRandomStream` (`self.Seed`)) 0 1)
        (:`0`
          (bind _output_get (set `local.currentAppendant` "1")))
        (:`1`
          (set `local.currentAppendant` "2")))
      (return (`KismetStringLibrary.Concat_StrStr` CurrentOrderString (`KismetTextLibrary.Conv_TextToString` _output_get) ". ")))
    (:`NewEnumerator1`
      ; ValueInsertion
      (switch `/Game/GameManage/DialogTables/E_OrderLineFormatterType` Type
        (:`NewEnumerator5`
          ;; Thematic Gen
          (bind _returnvalue (`|GetDataTableRow` (`self.ThematicDesctiptionDT`) Thematic)
            (:`then`
              (return (`KismetStringLibrary.Concat_StrStr` CurrentOrderString (`.ThemeDescription_2_68ADC1D8407432E673A962958B1D596F` (break `/Game/GameManage/ST_GroopedItems` _returnvalue)) ". ")))
            (:`RowNotFound`
              (bind _returnvalue_2 (`|GetDataTableRow` (`self.ThematicDesctiptionDTAll`) Thematic)
                (:`then`
                  (return (`KismetStringLibrary.Concat_StrStr` CurrentOrderString (`.ThemeDescription_2_68ADC1D8407432E673A962958B1D596F` (break `/Game/GameManage/ST_GroopedItems` _returnvalue_2)) ". ")))))))
        (:`NewEnumerator6`
          ;; Math gen
          (bind _outrownames (`DataTableFunctionLibrary.GetDataTableRowNames` _mathentrydialoguedt))
          (bind _returnvalue_3 (`|GetDataTableRow` _mathentrydialoguedt (`KismetArrayLibrary.Array_Random` _outrownames))
            (:`then`
              (bind _result (`/Game/GameManage/DialogTables/BP_TextLib.GetItemDeclension` MathRowName MathAmount))
              (return (`KismetStringLibrary.Concat_StrStr` CurrentOrderString " " (`KismetStringLibrary.Replace` (`.LineWithMask_3_3D97B67D480D281481769F8C53A56616` (break `/Game/GameManage/DialogTables/ST_DialMask` _returnvalue_3)) "*" (`KismetStringLibrary.Concat_StrStr` " " _result " ")))))))))
    (:`NewEnumerator2`
      (switch `int` (`KismetMathLibrary.RandomIntegerInRangeFromStream` (`KismetMathLibrary.MakeRandomStream` (`self.Seed`)) 0 1)
        (:`0`
          (bind _output_get_2 (set `local.currentAppendant` "1")))
        (:`1`
          (set `local.currentAppendant` "2")))
      (return (`KismetStringLibrary.Concat_StrStr` CurrentOrderString (`KismetTextLibrary.Conv_TextToString` _output_get_2))))
    (:`NewEnumerator3`)
    (:`NewEnumerator4`)))

(fn `Math2Generator`
  (params (ItemsCount :type Integer))
  (returns (GeneratedOrder :type "/Game/GameManage/ST_CustomerOrder Structure"))
  (locals (GeneratedItems :type Integer) (CurrentLine :type String))
  (bind _newparam (`self.GetAccessableSoloItems` ItemsCount))
  (bind _outitem (`KismetArrayLibrary.Array_Random` _newparam))
  (`|GetDataTableRow` "/Game/GameManage/DT_Items.DT_Items" _outitem
    (:`then`
      (`KismetArrayLibrary.Array_Add` (`.Items_24_92E324BF40B28E2E42823A94930C01BA` (break `/Game/GameManage/ST_CustomerOrder` (`self.GeneratedOrder`))) (make `/Game/GameManage/ST_GroopedItems` "Math elem" (`|MakeArray` (make `DataTableRowHandle` "/Game/GameManage/DT_Items.DT_Items" _outitem)) ItemsCount))
      (return))))

(fn `SuggestionGenerator`
  (returns (GeneratedOrder :type "/Game/GameManage/ST_CustomerOrder Structure"))
  (locals (NewItem :type "/Game/GameManage/ST_GroopedItems Structure"))
  (bind _generatedorder (`self.GeneratedOrder`))
  (bind _newitem_themedescription (break `/Game/GameManage/ST_GroopedItems` (`local.NewItem`)))
  (bind _groopedthemeitems (`self.GroopedThemeItems`))
  (`KismetSystemLibrary.PrintString` "1: SuggestionGen")
  (bind _newparam (`self.GetAccessableGroupedItems` _groopedthemeitems 1))
  (bind _returnvalue (`|GetDataTableRow` _groopedthemeitems (`KismetArrayLibrary.Array_RandomFromStream` _newparam (`KismetMathLibrary.MakeRandomStream` (`KismetMathLibrary.RandomInteger` 10000))))
    (:`then`
      (bind (_themedescription _itemsref) (break `/Game/GameManage/ST_GroopedItems` _returnvalue))
      (bind _output_get (set `local.NewItem` (make `/Game/GameManage/ST_GroopedItems` _themedescription _itemsref 1)))
      (`KismetArrayLibrary.Array_Add` (`.Items_24_92E324BF40B28E2E42823A94930C01BA` (break `/Game/GameManage/ST_CustomerOrder` _generatedorder)) _output_get)
      (set `self.GeneratedOrder` _generatedorder)
      (set `self.CurrentOrderString` (`KismetStringLibrary.Concat_StrStr` (`self.CurrentOrderString`) _newitem_themedescription))
      (return _generatedorder))))

(fn `UserConstructionScript`
  (bind _asbuild_shop_game_state (cast `/Game/BP_Main/BuildShopGameState` (`GameplayStatics.GetGameState`)))
  (set `self.BSGameStateRef` _asbuild_shop_game_state))