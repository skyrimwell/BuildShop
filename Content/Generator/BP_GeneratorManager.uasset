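; BP_GeneratorManager is an unfinished generator for a day's people count and their item purchases, using seeded random streams.
; StartDay rolls people and item totals, then sets a per-order cap that reserves one item for each other person.
; GenerateOrder rolls a purchase size and shrinks that cap.
; StartDay's GenerateOrder call sits behind an always-false condition, ComputeOrder is empty, and no event calls StartDay.
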(fn `ComputeOrder`)

(fn `GenerateOrder`
  (set `self.DailyCountOfBoughtItems_n` (`KismetMathLibrary.RandomIntegerInRangeFromStream` (`KismetMathLibrary.MakeRandomStream` (`self.Seed`)) (`self.MinBoughtItems`) (`self.MaxBoughtItems`)))
  (set `self.MaxBoughtItems` (- (+ (`self.MaxBoughtItems`) 1) (`self.DailyCountOfBoughtItems_n`))))

(fn `StartDay`
  (set `self.CountOfPeople` (`KismetMathLibrary.RandomIntegerInRangeFromStream` (`KismetMathLibrary.MakeRandomStream` (`self.Seed`)) (`self.MinPeople`) (`self.MaxPeople`)))
  (set `self.DailyCountOfItems` (`KismetMathLibrary.RandomIntegerInRangeFromStream` (`KismetMathLibrary.MakeRandomStream` (`self.Seed`)) (`self.MinItems`) (`self.MaxItems`)))
  (set `self.MaxBoughtItems` (- (+ (`self.DailyCountOfItems`) 1) (`self.CountOfPeople`)))
  (if (not true)
    (`self.GenerateOrder`)))

(fn `UserConstructionScript`)