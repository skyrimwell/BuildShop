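; Draggable component that lets the player drag a physics mesh with the mouse, constrained to a plane.
; On parent click, it grabs the mesh at the center of mass of the component under the cursor and takes CurrentAxis from BP_ShopPawn.
; Each tick moves the PhysicsHandle target to where the cursor ray intersects that axis actor's plane.
; Releasing the left mouse button drops the mesh and resets the handle target, intended to damp inertia.
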(event `OnParentClicked`
  (bind _returnvalue (`GameplayStatics.GetPlayerController` 0))
  (set `self.PC_Ref` _returnvalue)
  (`PhysicsHandleComponent.GrabComponentAtLocation` (`self.Physics Handle`) (`self.SM`) "None" (`PrimitiveComponent.GetCenterOfMass` (`.HitComponent` (`GameplayStatics.BreakHitResult` (`PlayerController.GetHitResultUnderCursorByChannel` _returnvalue "TraceTypeQuery1" true))) "None"))
  (set `self.isDragging` true)
  (bind _asbp_shop_pawn (cast `/Game/BP_Main/BP_ShopPawn` (`GameplayStatics.GetPlayerPawn` 0)))
  (set `self.Current Axis` (`/Game/BP_Main/BP_ShopPawn.CurrentAxis` _asbp_shop_pawn)))

(event `self.ReceiveTick`
  (params (DeltaSeconds :type "Float (single-precision)"))
  (bind _pc_ref (`self.PC_Ref`))
  (bind _current_axis (`self.Current Axis`))
  (bind (_locationx _locationy) (`PlayerController.GetMousePosition` _pc_ref))
  (bind (_worldposition _worlddirection) (`GameplayStatics.DeprojectScreenToWorld` _pc_ref (`KismetMathLibrary.MakeVector2D` _locationx _locationy)))
  (if (`self.isDragging`)
    (`PhysicsHandleComponent.SetTargetLocation` (`self.Physics Handle`) (`.Intersection` (`KismetMathLibrary.LinePlaneIntersection_OriginNormal` _worldposition (+ _worldposition (* _worlddirection 1000.0)) (`Actor.K2_GetActorLocation` _current_axis) (`Actor.GetActorUpVector` _current_axis))))
    ;[1 1 1] Выход из стейта захвата
    (if (not (`PlayerController.IsInputKeyDown` (`self.PC_Ref`) "LeftMouseButton"))
      (`PhysicsHandleComponent.ReleaseComponent` (`self.Physics Handle`))
      (set `self.isDragging` false)
      ;[1 1 1] Гашение инерции
      (`PhysicsHandleComponent.SetTargetLocation` (`self.Physics Handle`) (`SceneComponent.RelativeLocation` (`self.SM`)))
      (`KismetSystemLibrary.Delay` 0.5))))