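; Player pawn for a shop game that serves as a movable viewpoint and launches shop UI.
; Events snap it between placed point actors for cashier, storage, turned view, decor and register, tracking location state with flags.
; Storage shows a delayed return button; register mode initializes the controller's interface after a delay and resets RegisterChanger on exit.
; It also opens purchase and outlay widgets, chaining purchase menu removal into assortment expansion.
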(event `self.ReceiveBeginPlay`
  (set `self.AtTheStorage` false)
  (bind _asshop_player_controller (cast `/Game/BP_Main/ShopPlayerController` (`GameplayStatics.GetPlayerController` 0)))
  (set `self.PCRef` _asshop_player_controller))

(event `MoveToCass`
  (`self.K2_SetActorTransform` (`self.GetTransform` (`self.CassPoint`)) false true)
  (set `self.AtTheStorage` false)
  ; TurnAround
  (`Widget.RemoveFromParent` (`self.TurnBtn`)))

(event `MoveToStore`
  (`self.K2_SetActorTransform` (`self.GetTransform` (`self.StorePoint`)) false true)
  (set `self.AtTheStorage` true)
  ; TurnAround
  (bind _returnvalue (`|CreateWidget` "/Game/Storage/ReturnBtn.ReturnBtn_C"))
  (set `self.TurnBtn` _returnvalue)
  (`KismetSystemLibrary.Delay` 2.0)
  (`UserWidget.AddToViewport` _returnvalue 0))

(event `StartPurchaseEvent`
  (bind _returnvalue (`|CreateWidget` "/Game/ItemOrderingSystem/WBP_PurchaseMenu.WBP_PurchaseMenu_C" (`GameplayStatics.GetPlayerController` 0) "/Game/GameManage/DT_Items.DT_Items"))
  (`UserWidget.AddToViewport` _returnvalue 0)
  (add `/Game/ItemOrderingSystem/WBP_PurchaseMenu.OnRemove` _returnvalue (delegate `StartAssortmentExpandingEvent`)))

(event `TurnAround`
  (bind (_returnvalue_location _returnvalue_rotation _returnvalue_scale) (`KismetMathLibrary.BreakTransform` (`self.GetTransform` (`self.SecondPoint`))))
  ; TurnAround
  (set `self.bIsTurned` true)
  (`self.K2_SetActorTransform` (`KismetMathLibrary.MakeTransform` _returnvalue_location _returnvalue_rotation _returnvalue_scale)))

(event `MoveToDecorPart`
  (`self.K2_SetActorTransform` (`self.GetTransform` (`self.DecorPoint`)) false true))

(event `Advance DayTime`)

(event `StorageReturn`
  ; TurnAround
  (set `self.bIsTurned` false)
  (`self.K2_SetActorTransform` (`self.GetTransform` (`self.StorePoint`))))

(event `StartConfirmOutlayEvent`
  (bind _returnvalue (`|CreateWidget` "/Game/ItemOrderingSystem/WBP_Outlay.WBP_Outlay_C" (`GameplayStatics.GetPlayerController` 0) true))
  (`UserWidget.AddToViewport` _returnvalue 0))

(event `RegisterInit`
  (set `self.bIsRegisterMode` true)
  (`self.K2_SetActorTransform` (`self.GetTransform` (`self.RegisterPoint`)))
  ; Анимация зума к кассе
  (`KismetSystemLibrary.Delay` 2.0)
  (`/Game/Widgets/WBP_PlayerInterface.InitRegisterMode` (`/Game/BP_Main/ShopPlayerController.PlayerInterface` (`self.PCRef`))))

(event `StartAssortmentExpandingEvent`
  (bind _returnvalue (`|CreateWidget` "/Game/ItemOrderingSystem/WBP_AssortmentExpansion.WBP_AssortmentExpansion_C" (`GameplayStatics.GetPlayerController` 0)))
  (`UserWidget.AddToViewport` _returnvalue 0))

(event `RegisterExit`
  (set `self.bIsRegisterMode` false)
  (`self.K2_SetActorTransform` (`self.GetTransform` (`self.CassPoint`)))
  (`/Game/CashRegister/BP_RegisterCameraChanger.ReturnToBase` (`self.RegisterChanger`)))

(fn `UserConstructionScript`)