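; BP_CashRegisterCheck is the draggable check at the cash register, which the player drops into a check zone to be compared.
; BeginPlay hands its mesh and PhysicsHandle to BPDraggableComponent, which receives clicks on the actor.
; On release inside CheckZoneRef it calls CompareCheck through GSRef.
; Otherwise it disables physics, waits one tick and teleports back to its standby transform.
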(event `/Game/BP_Main/BPI_Clickable1.OnObjectReleased`
  (params (IsHolded :type Boolean))
  (bind _bischeckinside (`/Game/CashRegister/BP_CheckZone.bIsCheckInside` (`self.CheckZoneRef`)))
  (if _bischeckinside
    (`/Game/BP_Main/BuildShopGameState.CompareCheck` (`self.GSRef`))
    (else
      ; Возврат на базу
      (`KismetSystemLibrary.PrintString` (`KismetStringLibrary.Conv_BoolToString` _bischeckinside))
      (`PrimitiveComponent.SetSimulatePhysics` (`self.CheckSM`) false)
      (`KismetSystemLibrary.DelayUntilNextTick`)
      (`self.K2_SetActorTransform` (`self.CheckStandbyCoords`) false true))))

(event `/Game/BP_Main/BPI_Clickable1.OnObjectClicked`
  (`/Game/BP_Main/BP_DraggableComponent.OnParentClicked` (`self.BP_DraggableComponent`))
  (`KismetSystemLibrary.PrintString` "Hello"))

(event `self.ReceiveBeginPlay`
  (bind _bp_draggablecomponent (`self.BP_DraggableComponent`))
  (set `/Game/BP_Main/BP_DraggableComponent.SM` (`self.CheckSM`) _bp_draggablecomponent)
  (set `/Game/BP_Main/BP_DraggableComponent.Physics Handle` (`self.PhysicsHandle`) _bp_draggablecomponent))

(fn `UserConstructionScript`)