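; Clickable 3D cash register keypad with digit, Clear and Delete buttons that report presses through event dispatchers.
; Component click events route to press events, each using a timeline to lerp the clicked button's relative Z downward.
; A shared IsLocked flag ignores clicks during the animation.
; The matching dispatcher fires only when the timeline finishes, with digit presses passing an enum value.
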(event `PressBtn`
  (params (WhatPresed :type "PrimitiveComponent Object Reference") (BtnEnum :type "/Game/CashRegister/E_CashRegisterBtn Enum" :default "NewEnumerator0"))
  (bind (_relativelocation_x _relativelocation_y) (`KismetMathLibrary.BreakVector` (`SceneComponent.RelativeLocation` WhatPresed)))
  (bind (_relativelocation_x_2 _relativelocation_y_2 _relativelocation_z) (`KismetMathLibrary.BreakVector` (`SceneComponent.RelativeLocation` WhatPresed)))
  (if (not (`self.bIsLocked`))
    (bind _output_get (set `self.StoredZ` _relativelocation_z))
    (set `self.bIsLocked` true)
    (bind (_direction _pressvolume) (`Timeline|MoveBtn` :!via `PlayFromStart`)
      (:`Update`
        (`SceneComponent.K2_SetRelativeLocation` WhatPresed (`KismetMathLibrary.MakeVector` _relativelocation_x _relativelocation_y (`KismetMathLibrary.Lerp` _output_get (- _output_get 2.0) _pressvolume)) false false))
      (:`Finished`
        (set `self.bIsLocked` false)
        (`self.OnDigitPressed` BtnEnum)))))

(event `self.BTN0.OnClicked`
  (params (TouchedComponent :type "PrimitiveComponent Object Reference") (ButtonPressed :type "Key Structure"))
  (if (not (`self.bIsLocked`))
    (`self.PressBtn` TouchedComponent)))

(event `self.BTN1.OnClicked`
  (params (TouchedComponent :type "PrimitiveComponent Object Reference") (ButtonPressed :type "Key Structure"))
  (if (not (`self.bIsLocked`))
    (`self.PressBtn` TouchedComponent "NewEnumerator1")))

(event `PressClear`
  (params (WhatPresed :type "PrimitiveComponent Object Reference"))
  (bind (_relativelocation_x _relativelocation_y) (`KismetMathLibrary.BreakVector` (`SceneComponent.RelativeLocation` WhatPresed)))
  (bind (_relativelocation_x_2 _relativelocation_y_2 _relativelocation_z) (`KismetMathLibrary.BreakVector` (`SceneComponent.RelativeLocation` WhatPresed)))
  (if (not (`self.bIsLocked`))
    (bind _output_get (set `self.StoredZ` _relativelocation_z))
    (set `self.bIsLocked` true)
    (bind (_direction _pressvolume) (`Timeline|Timeline` :!via `PlayFromStart`)
      (:`Update`
        (`SceneComponent.K2_SetRelativeLocation` WhatPresed (`KismetMathLibrary.MakeVector` _relativelocation_x _relativelocation_y (`KismetMathLibrary.Lerp` _output_get (- _output_get 2.0) _pressvolume)) false false))
      (:`Finished`
        (set `self.bIsLocked` false)
        (`self.OnClearPressed`)))))

(event `self.BTN2.OnClicked`
  (params (TouchedComponent :type "PrimitiveComponent Object Reference") (ButtonPressed :type "Key Structure"))
  (if (not (`self.bIsLocked`))
    (`self.PressBtn` TouchedComponent "NewEnumerator2")))

(event `self.BTN3.OnClicked`
  (params (TouchedComponent :type "PrimitiveComponent Object Reference") (ButtonPressed :type "Key Structure"))
  (if (not (`self.bIsLocked`))
    (`self.PressBtn` TouchedComponent "NewEnumerator3")))

(event `self.BTN4.OnClicked`
  (params (TouchedComponent :type "PrimitiveComponent Object Reference") (ButtonPressed :type "Key Structure"))
  (if (not (`self.bIsLocked`))
    (`self.PressBtn` TouchedComponent "NewEnumerator4")))

(event `self.BTN5.OnClicked`
  (params (TouchedComponent :type "PrimitiveComponent Object Reference") (ButtonPressed :type "Key Structure"))
  (if (not (`self.bIsLocked`))
    (`self.PressBtn` TouchedComponent "NewEnumerator5")))

(event `PressDelete`
  (params (WhatPresed :type "PrimitiveComponent Object Reference"))
  (bind (_relativelocation_x _relativelocation_y) (`KismetMathLibrary.BreakVector` (`SceneComponent.RelativeLocation` WhatPresed)))
  (bind (_relativelocation_x_2 _relativelocation_y_2 _relativelocation_z) (`KismetMathLibrary.BreakVector` (`SceneComponent.RelativeLocation` WhatPresed)))
  (if (not (`self.bIsLocked`))
    (bind _output_get (set `self.StoredZ` _relativelocation_z))
    (set `self.bIsLocked` true)
    (bind (_direction _pressvolume) (`Timeline|Timeline_0` :!via `PlayFromStart`)
      (:`Update`
        (`SceneComponent.K2_SetRelativeLocation` WhatPresed (`KismetMathLibrary.MakeVector` _relativelocation_x _relativelocation_y (`KismetMathLibrary.Lerp` _output_get (- _output_get 2.0) _pressvolume)) false false))
      (:`Finished`
        (set `self.bIsLocked` false)
        (`self.OnDeletePressed`)))))

(event `self.BTN6.OnClicked`
  (params (TouchedComponent :type "PrimitiveComponent Object Reference") (ButtonPressed :type "Key Structure"))
  (if (not (`self.bIsLocked`))
    (`self.PressBtn` TouchedComponent "NewEnumerator6")))

(event `self.BTN7.OnClicked`
  (params (TouchedComponent :type "PrimitiveComponent Object Reference") (ButtonPressed :type "Key Structure"))
  (if (not (`self.bIsLocked`))
    (`self.PressBtn` TouchedComponent "NewEnumerator7")))

(event `self.BTN8.OnClicked`
  (params (TouchedComponent :type "PrimitiveComponent Object Reference") (ButtonPressed :type "Key Structure"))
  (if (not (`self.bIsLocked`))
    (`self.PressBtn` TouchedComponent "NewEnumerator8")))

(event `self.BTN9.OnClicked`
  (params (TouchedComponent :type "PrimitiveComponent Object Reference") (ButtonPressed :type "Key Structure"))
  (if (not (`self.bIsLocked`))
    (`self.PressBtn` TouchedComponent "NewEnumerator9")))

(event `self.BTNClear.OnClicked`
  (params (TouchedComponent :type "PrimitiveComponent Object Reference") (ButtonPressed :type "Key Structure"))
  (if (not (`self.bIsLocked`))
    (`self.PressClear` TouchedComponent)))

(event `self.BTNDelete.OnClicked`
  (params (TouchedComponent :type "PrimitiveComponent Object Reference") (ButtonPressed :type "Key Structure"))
  (if (not (`self.bIsLocked`))
    (`self.PressDelete` TouchedComponent)))

(fn `UserConstructionScript`)