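; Cash register camera changer actor that provides a clickable box for switching the shop pawn into register mode.
; It caches the player's shop pawn on BeginPlay, then clicking the box calls that pawn's register initialisation.
; The click also teleports the box to an out-of-the-way marker position, and a ReturnToBase event moves it back to its visible marker.
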(event `self.ReceiveBeginPlay`
  (bind _asbp_shop_pawn (cast `/Game/BP_Main/BP_ShopPawn` (`GameplayStatics.GetPlayerPawn` 0)))
  (set `self.PawnRef` _asbp_shop_pawn))

(event `self.Box.OnClicked`
  (params (TouchedComponent :type "PrimitiveComponent Object Reference") (ButtonPressed :type "Key Structure"))
  (`/Game/BP_Main/BP_ShopPawn.RegisterInit` (`self.PawnRef`))
  (`SceneComponent.K2_SetRelativeLocation` (`self.Box`) (`SceneComponent.RelativeLocation` (`self.PlaceOut`)) false true))

(event `ReturnToBase`
  (`SceneComponent.K2_SetRelativeLocation` (`self.Box`) (`SceneComponent.RelativeLocation` (`self.PlaceVisible`)) false true))

(fn `UserConstructionScript`)