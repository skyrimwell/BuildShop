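; Order box actor that holds delivered items and presents them through a tooltip widget when clicked.
; AddItems copies map values into StoredItems and re-arms the box, so the next click opens a WBP_ToolTip projected above it.
; GetNextItem pops the first item into the tooltip, which also receives a reference to the box.
; Box overlaps track entering and leaving items, and releasing commits any non-empty PotentialItem.
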(event `self.ReceiveBeginPlay`
  (set `self.IsBoxOpened` true))

(event `AddItems`
  (params (ItemsToAdd :type "Map of Integer to /Game/GameManage/ST_ItemStack Structure"))
  (bind _keys (`BlueprintMapLibrary.Map_Keys` ItemsToAdd))
  (for _array_element _keys
    (`KismetArrayLibrary.Array_Add` (`self.StoredItems`) (`BlueprintMapLibrary.Map_Find` ItemsToAdd _array_element)))
  (set `self.IsBoxOpened` false))

(event `CreateTooltip`
  (bind (_returnvalue_x _returnvalue_y) (`KismetMathLibrary.BreakVector2D` (`WidgetLayoutLibrary.GetViewportSize`)))
  (bind (_origin _boxextent) (`self.GetActorBounds` self false false))
  (bind _returnvalue (`|CreateWidget` "/Game/Storage/WBP_ToolTip.WBP_ToolTip_C"))
  (set `self.ToolTipRef` _returnvalue)
  (`UserWidget.SetPositionInViewport` _returnvalue (`GameplayStatics.ProjectWorldToScreen` (`GameplayStatics.GetPlayerController` 0) (+ _origin (`KismetMathLibrary.MakeVector` 0.0 0.0 (* (.z _boxextent) 2.0))) true) true)
  (`UserWidget.SetDesiredSizeInViewport` _returnvalue (`KismetMathLibrary.MakeVector2D` (/ _returnvalue_x 10.0) (/ _returnvalue_y 5.0)))
  (`UserWidget.AddToViewport` _returnvalue 0)
  (`self.GetNextItem`)
  (set `/Game/Storage/WBP_ToolTip.OrderBox` self (`self.ToolTipRef`)))

(event `/Game/BP_Main/BPI_Clickable1.OnObjectClicked`
  (if (not (`self.IsBoxOpened`))
    (`self.CreateTooltip`)
    (set `self.IsBoxOpened` true)))

(event `self.Box.OnComponentBeginOverlap`
  (params (OverlappedComponent :type "PrimitiveComponent Object Reference") (OtherActor :type "Actor Object Reference") (OtherComp :type "PrimitiveComponent Object Reference") (OtherBodyIndex :type Integer) (bFromSweep :type Boolean) (SweepResult :type "HitResult Structure (by ref)"))
  (`self.OnItemEnter` OtherActor))

(event `self.Box.OnComponentEndOverlap`
  (params (OverlappedComponent :type "PrimitiveComponent Object Reference") (OtherActor :type "Actor Object Reference") (OtherComp :type "PrimitiveComponent Object Reference") (OtherBodyIndex :type Integer))
  (`self.OnItemOut` OtherActor))

(event `/Game/BP_Main/BPI_Clickable1.OnObjectReleased`
  (params (IsHolded :type Boolean))
  (if (!= (`.ItemQuantity_4_F5DAE9484DE62FBE49B5F0A69999838A` (break `/Game/GameManage/ST_ItemStack` (`self.Potential Item`))) 0)
    (`self.Add potential item`)))

(event `self.OnAddItem`
  (params (Item :type "/Game/GameManage/ST_ItemStack Structure"))
  (`KismetArrayLibrary.Array_Add` (`self.StoredItems`) Item))

(fn `GetNextItem`
  (bind _storeditems (`self.StoredItems`))
  (if (!= (`KismetArrayLibrary.Array_Length` (`self.StoredItems`)) 0)
    (`/Game/Storage/WBP_ToolTip.SetToolTipInfo` (`self.ToolTipRef`) (`|GetArrayItem` _storeditems))
    (`KismetArrayLibrary.Array_Remove` _storeditems)))

(fn `UserConstructionScript`)