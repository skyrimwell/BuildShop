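; Storage slot actor for a shop-building game that holds one item stack, seeded randomly from BuildShopGameState at BeginPlay.
; A box overlap feeds item enter/exit handling; adding an item merges matching IDs, otherwise ejects the old stack as BP_StoredItem.
; Holding the slot dispenses one item, while the WBP_StoreWidget take button spawns the whole stack.
; Changes refresh the widget; adds and single withdrawals also update the game state.
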(event `/Game/BP_Main/BPI_Clickable1.OnObjectReleased`
  (params (IsHolded :type Boolean))
  (if (not IsHolded)
    (bind _aswbp_store_widget (cast `/Game/Widgets/WBP_StoreWidget` (`WidgetComponent.GetWidget` (`self.Widget`))))
    (bind _widgetref (`/Game/Widgets/WBP_StoreWidget.Set Slot Ref` _aswbp_store_widget self))
    (`UserWidget.AddToViewport` _widgetref 0)))

(event `HideWidget`
  ;[1 1 1] Old
  (`SceneComponent.SetVisibility` (`self.Widget`) false false))

(event `self.ReceiveBeginPlay`
  (`|ExecutionSequence`
    (:`then_0`
      (bind _aswbp_store_widget (cast `/Game/Widgets/WBP_StoreWidget` (`WidgetComponent.GetWidget` (`self.Widget`))))
      (add `Button.OnPressed` (`/Game/Widgets/WBP_StoreWidget.ExitButton` _aswbp_store_widget) (delegate `HideWidget`))
      (`SceneComponent.SetVisibility` (`self.Widget`) false false))
    (:`then_1`
      (add `Button.OnClicked` (`/Game/Widgets/WBP_StoreWidget.TakeButton` _aswbp_store_widget) (delegate `TakeItem`)))
    (:`then_2`
      (bind _asbuild_shop_game_state (cast `/Game/BP_Main/BuildShopGameState` (`GameplayStatics.GetGameState`)))
      (bind _newparam (`/Game/BP_Main/BuildShopGameState.GetRandomItem` _asbuild_shop_game_state))
      (set `self.LastStoredItemStack` _newparam)
      (`self.UpdateUI`)
      (`KismetSystemLibrary.PrintString` "Hello"))))

(event `TakeItem`
  (bind _laststoreditemstack (`self.LastStoredItemStack`))
  (bind (_laststoreditemstack_item _laststoreditemstack_itemquantity) (break `/Game/GameManage/ST_ItemStack` (`self.LastStoredItemStack`)))
  (`KismetSystemLibrary.PrintText` (`KismetTextLibrary.Conv_StringToText` (`KismetStringLibrary.Concat_StrStr` (`KismetStringLibrary.Conv_NameToString` (break `/Game/GameManage/ST_Item` (break `/Game/GameManage/ST_ItemStack` _laststoreditemstack))) "" (`KismetStringLibrary.Conv_IntToString` (`.ItemID_10_05E1392B4735FFE91395E096C0362B11` (break `/Game/GameManage/ST_Item` (break `/Game/GameManage/ST_ItemStack` _laststoreditemstack)))) "" (`KismetSystemLibrary.GetDisplayName` (`.Sprite_12_C3E3BEF7482375E8B6ED59A9B46A7A49` (break `/Game/GameManage/ST_Item` (break `/Game/GameManage/ST_ItemStack` _laststoreditemstack)))) "" (`KismetStringLibrary.Conv_IntToString` (`.DisplayCode_14_DA320A0F46F774CC85313AB0D355DB03` (break `/Game/GameManage/ST_Item` (break `/Game/GameManage/ST_ItemStack` _laststoreditemstack)))) "" (`KismetStringLibrary.Conv_DoubleToString` (`.ItemCost_20_EF3CC9BC4D8F1FE198FCE58B55A35F26` (break `/Game/GameManage/ST_Item` (break `/Game/GameManage/ST_ItemStack` _laststoreditemstack)))) "" (`KismetStringLibrary.Conv_IntToString` (`.ItemQuantity_4_F5DAE9484DE62FBE49B5F0A69999838A` (break `/Game/GameManage/ST_ItemStack` _laststoreditemstack))))))
  (if (!= 0 _laststoreditemstack_itemquantity)
    (bind _returnvalue (`|SpawnActorFromClass` "/Game/Storage/BP_StoredItem.BP_StoredItem_C" (`SceneComponent.K2_GetComponentToWorld` (`self.SpawnPointSC`)) "AlwaysSpawn" "MultiplyWithRoot" null null null))
    (set `/Game/Storage/BP_StoredItem.ItemInfo` (`self.LastStoredItemStack`) _returnvalue)
    (set `self.LastStoredItemStack` (struct))
    (`self.UpdateUI`)
    (else
      (`KismetSystemLibrary.PrintText` "Nothing here"))))

(event `UpdateUI`
  (bind _laststoreditemstack (`self.LastStoredItemStack`))
  (bind _aswbp_store_widget (cast `/Game/Widgets/WBP_StoreWidget` (`WidgetComponent.GetWidget` (`self.Widget`))))
  (`/Game/Widgets/WBP_StoreWidget.Set Item Stats` _aswbp_store_widget (`.Sprite_12_C3E3BEF7482375E8B6ED59A9B46A7A49` (break `/Game/GameManage/ST_Item` (break `/Game/GameManage/ST_ItemStack` _laststoreditemstack))) (`KismetTextLibrary.Conv_NameToText` (break `/Game/GameManage/ST_Item` (break `/Game/GameManage/ST_ItemStack` _laststoreditemstack))) (`.ItemID_10_05E1392B4735FFE91395E096C0362B11` (break `/Game/GameManage/ST_Item` (break `/Game/GameManage/ST_ItemStack` _laststoreditemstack))) (`.DisplayCode_14_DA320A0F46F774CC85313AB0D355DB03` (break `/Game/GameManage/ST_Item` (break `/Game/GameManage/ST_ItemStack` _laststoreditemstack))) (`.ItemQuantity_4_F5DAE9484DE62FBE49B5F0A69999838A` (break `/Game/GameManage/ST_ItemStack` _laststoreditemstack))))

(event `/Game/BP_Main/BPI_Clickable1.OnObjectHolded`
  (bind (_laststoreditemstack_item _laststoreditemstack_itemquantity) (break `/Game/GameManage/ST_ItemStack` (`self.LastStoredItemStack`)))
  (bind _laststoreditemstack_item_2 (break `/Game/GameManage/ST_ItemStack` (`self.LastStoredItemStack`)))
  (if (not (== _laststoreditemstack_itemquantity 0))
    (set `self.LastStoredItemStack` (make `/Game/GameManage/ST_ItemStack` _laststoreditemstack_item (- _laststoreditemstack_itemquantity 1)))
    (bind _returnvalue (`|SpawnActorFromClass` "/Game/Storage/BP_StoredItem.BP_StoredItem_C" (`SceneComponent.K2_GetComponentToWorld` (`self.SpawnPointSC`)) "AlwaysSpawn" "MultiplyWithRoot" null null null))
    (set `/Game/Storage/BP_StoredItem.ItemInfo` (make `/Game/GameManage/ST_ItemStack` _laststoreditemstack_item_2 1) _returnvalue)
    (`self.UpdateUI`)
    (bind _asbuild_shop_game_state (cast `/Game/BP_Main/BuildShopGameState` (`GameplayStatics.GetGameState`)))
    (`/Game/BP_Main/BuildShopGameState.UpdateStorageSlot` _asbuild_shop_game_state self (`self.LastStoredItemStack`))))

(event `self.OnAddItem`
  (params (Item :type "/Game/GameManage/ST_ItemStack Structure"))
  (bind _potential_item (`self.Potential Item`))
  (bind _potential_item_item (break `/Game/GameManage/ST_ItemStack` (`self.Potential Item`)))
  (bind (_item _itemquantity) (break `/Game/GameManage/ST_ItemStack` (`self.LastStoredItemStack`)))
  (if (== (`.ItemID_10_05E1392B4735FFE91395E096C0362B11` (break `/Game/GameManage/ST_Item` _item)) (`.ItemID_10_05E1392B4735FFE91395E096C0362B11` (break `/Game/GameManage/ST_Item` (break `/Game/GameManage/ST_ItemStack` _potential_item))))
    (set `self.LastStoredItemStack` (make `/Game/GameManage/ST_ItemStack` _potential_item_item (+ _itemquantity (`.ItemQuantity_4_F5DAE9484DE62FBE49B5F0A69999838A` (break `/Game/GameManage/ST_ItemStack` _potential_item)))))
    (`/Game/BP_Main/BuildShopGameState.UpdateStorageSlot` (stale _asbuild_shop_game_state) self (`self.LastStoredItemStack`))
    (`self.UpdateUI`)
    (else
      (if (not (== _itemquantity 0))
        (bind _returnvalue (`|SpawnActorFromClass` "/Game/Storage/BP_StoredItem.BP_StoredItem_C" (`SceneComponent.K2_GetComponentToWorld` (`self.SpawnPointSC`)) "AlwaysSpawn" "MultiplyWithRoot" null null null))
        (set `/Game/Storage/BP_StoredItem.ItemInfo` (`self.LastStoredItemStack`) _returnvalue))
      (set `self.LastStoredItemStack` (`self.Potential Item`))
      (bind _asbuild_shop_game_state (cast `/Game/BP_Main/BuildShopGameState` (`GameplayStatics.GetGameState`)))
      (`/Game/BP_Main/BuildShopGameState.UpdateStorageSlot` _asbuild_shop_game_state self (`self.LastStoredItemStack`))
      (`self.UpdateUI`))))

(event `self.Box.OnComponentBeginOverlap`
  (params (OverlappedComponent :type "PrimitiveComponent Object Reference") (OtherActor :type "Actor Object Reference") (OtherComp :type "PrimitiveComponent Object Reference") (OtherBodyIndex :type Integer) (bFromSweep :type Boolean) (SweepResult :type "HitResult Structure (by ref)"))
  (`self.OnItemEnter` OtherActor))

(event `self.Box.OnComponentEndOverlap`
  (params (OverlappedComponent :type "PrimitiveComponent Object Reference") (OtherActor :type "Actor Object Reference") (OtherComp :type "PrimitiveComponent Object Reference") (OtherBodyIndex :type Integer))
  (`self.OnItemOut` OtherActor))

(fn `UserConstructionScript`)