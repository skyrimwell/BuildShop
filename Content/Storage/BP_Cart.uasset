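; Draggable physics shopping cart that carries a list of items and travels with the player between the storage and the checkout (Cass).
; Clicks go to BPDraggableComponent, while its Box reports items entering or leaving and flags readiness when touching BP_Door.
; Releasing it at the door moves BP_ShopPawn and teleports the cart, toggling physics across a tick.
; Otherwise, a non-held release opens WBP_CartInterface listing CartArray; the CartStorage map logic is disconnected.
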(event `ClearCart`
  (`KismetArrayLibrary.Array_Clear` (`self.CartArray`)))

(event `self.ReceiveBeginPlay`
  (bind _bp_draggablecomponent (`self.BP_DraggableComponent`))
  (set `/Game/BP_Main/BP_DraggableComponent.Physics Handle` (`self.PhysicsHandle`) _bp_draggablecomponent)
  (set `/Game/BP_Main/BP_DraggableComponent.SM` (`self.StaticMesh`) _bp_draggablecomponent)
  (bind _returnvalue (`GameplayStatics.GetActorOfClass` "/Game/ShopMap/BP_Door.BP_Door_C"))
  (set `self.DoorReference` _returnvalue)
  (set `self.ReadyToGo` false))

(event `self.OnAddItem`
  (params (Item :type "/Game/GameManage/ST_ItemStack Structure"))
  (`KismetArrayLibrary.Array_Add` (`self.CartArray`) Item))

(event `ShowCart`
  (bind _cartstorage (`self.CartStorage`))
  (bind _keys (`BlueprintMapLibrary.Map_Keys` _cartstorage))
  (for _array_element _keys
    (bind _value (`BlueprintMapLibrary.Map_Find` _cartstorage _array_element))
    (`KismetSystemLibrary.PrintString` (`KismetStringLibrary.Concat_StrStr` "___________ \n" (`KismetStringLibrary.Conv_NameToString` (break `/Game/GameManage/ST_Item` (break `/Game/GameManage/ST_ItemStack` _value))) " \nКоличество:" (`KismetStringLibrary.Conv_IntToString` (`.ItemQuantity_4_F5DAE9484DE62FBE49B5F0A69999838A` (break `/Game/GameManage/ST_ItemStack` _value))) "-------------- \n"))))

(event `/Game/BP_Main/BPI_Clickable1.OnObjectClicked`
  (`/Game/BP_Main/BP_DraggableComponent.OnParentClicked` (`self.BP_DraggableComponent`)))

(event `self.Box.OnComponentBeginOverlap`
  (params (OverlappedComponent :type "PrimitiveComponent Object Reference") (OtherActor :type "Actor Object Reference") (OtherComp :type "PrimitiveComponent Object Reference") (OtherBodyIndex :type Integer) (bFromSweep :type Boolean) (SweepResult :type "HitResult Structure (by ref)"))
  (`self.OnItemEnter` OtherActor)
  (if (== (`self.DoorReference`) OtherActor)
    (set `self.ReadyToGo` true)
    (`KismetSystemLibrary.PrintString` "IsReady")))

(event `self.Box.OnComponentEndOverlap`
  (params (OverlappedComponent :type "PrimitiveComponent Object Reference") (OtherActor :type "Actor Object Reference") (OtherComp :type "PrimitiveComponent Object Reference") (OtherBodyIndex :type Integer))
  (`self.OnItemOut` OtherActor)
  (if (== (`self.DoorReference`) OtherActor)
    (set `self.ReadyToGo` false)
    (`KismetSystemLibrary.PrintString` "Isn't Ready")))

(event `/Game/BP_Main/BPI_Clickable1.OnObjectReleased`
  (params (IsHolded :type Boolean))
  (if (`self.ReadyToGo`)
    (bind _asbp_shop_pawn (cast `/Game/BP_Main/BP_ShopPawn` (`GameplayStatics.GetPlayerPawn` 0)))
    (if (`/Game/BP_Main/BP_ShopPawn.AtTheStorage` _asbp_shop_pawn)
      (`/Game/BP_Main/BP_ShopPawn.MoveToCass` _asbp_shop_pawn)
      (`self.BringCartToCass`)
      (else
        (`/Game/BP_Main/BP_ShopPawn.MoveToStore` _asbp_shop_pawn)
        (`self.BringCartToStorage`)))
    (elif (not IsHolded)
      (bind _returnvalue (`|CreateWidget` "/Game/Storage/WBP_CartInterface.WBP_CartInterface_C" (`GameplayStatics.GetPlayerController` 0)))
      (`UserWidget.AddToViewport` _returnvalue 0)
      (for _array_element (`self.CartArray`)
        (`/Game/Storage/WBP_CartInterface.AddItem` _returnvalue _array_element)))))

(event `BringCartToCass`
  (bind (_returnvalue_location _returnvalue_rotation) (`KismetMathLibrary.BreakTransform` (`self.GetTransform` (`self.CassPoint`))))
  (`PrimitiveComponent.SetSimulatePhysics` (`self.StaticMesh`) false)
  (`KismetSystemLibrary.DelayUntilNextTick`)
  (`SceneComponent.K2_SetRelativeLocationAndRotation` (`self.StaticMesh`) _returnvalue_location _returnvalue_rotation false false)
  (`PrimitiveComponent.SetSimulatePhysics` (`self.StaticMesh`) true))

(event `BringCartToStorage`
  (bind (_returnvalue_location _returnvalue_rotation) (`KismetMathLibrary.BreakTransform` (`self.GetTransform` (`self.StoragePoint`))))
  (`PrimitiveComponent.SetSimulatePhysics` (`self.StaticMesh`) false)
  (`KismetSystemLibrary.DelayUntilNextTick`)
  (`SceneComponent.K2_SetRelativeLocationAndRotation` (`self.StaticMesh`) _returnvalue_location _returnvalue_rotation false false)
  (`PrimitiveComponent.SetSimulatePhysics` (`self.StaticMesh`) true))

(fn `UserConstructionScript`
  (`parent.UserConstructionScript`))