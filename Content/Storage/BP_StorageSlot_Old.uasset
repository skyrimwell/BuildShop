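; Storage slot actor that holds one item stack and shows it in a WBP_StoreWidget when clicked.
; The widget's stats are filled only at BeginPlay; its Take button spawns the stack as a BP_StoredItem and empties the slot.
; Overlapping actors receive preview messages and return a candidate stack.
; AddItem merges stacks with matching IDs, otherwise ejects any stored stack as a spawned item and stores the new one.
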(event `/Game/BP_Main/BPI_Clickable1.OnObjectClicked`
  (bind _widget (`self.Widget`))
  (if (not (`SceneComponent.bVisible` _widget))
    (`SceneComponent.SetVisibility` _widget true true)))

(event `HideWidget`
  (`SceneComponent.SetVisibility` (`self.Widget`) false true))

(event `self.ReceiveBeginPlay`
  (bind _storeditemstack (`self.StoredItemStack`))
  (`|ExecutionSequence`
    (:`then_0`
      (bind _aswbp_store_widget (cast `/Game/Widgets/WBP_StoreWidget` (`WidgetComponent.GetWidget` (`self.Widget`))))
      (add `Button.OnPressed` (`/Game/Widgets/WBP_StoreWidget.ExitButton` _aswbp_store_widget) (delegate `HideWidget`))
      (`SceneComponent.SetVisibility` (`self.Widget`) false false)
      (bind _aswbp_store_widget_2 (cast `/Game/Widgets/WBP_StoreWidget` (`WidgetComponent.GetWidget` (`self.Widget`))))
      (`/Game/Widgets/WBP_StoreWidget.Set Item Stats` _aswbp_store_widget_2 (`.Sprite_12_C3E3BEF7482375E8B6ED59A9B46A7A49` (break `/Game/GameManage/ST_Item` (break `/Game/GameManage/ST_ItemStack` _storeditemstack))) (`KismetTextLibrary.Conv_NameToText` (break `/Game/GameManage/ST_Item` (break `/Game/GameManage/ST_ItemStack` _storeditemstack))) (`.ItemID_10_05E1392B4735FFE91395E096C0362B11` (break `/Game/GameManage/ST_Item` (break `/Game/GameManage/ST_ItemStack` _storeditemstack))) (`.DisplayCode_14_DA320A0F46F774CC85313AB0D355DB03` (break `/Game/GameManage/ST_Item` (break `/Game/GameManage/ST_ItemStack` _storeditemstack))) (`.ItemQuantity_4_F5DAE9484DE62FBE49B5F0A69999838A` (break `/Game/GameManage/ST_ItemStack` _storeditemstack)))
      (`KismetSystemLibrary.PrintText` "Hello"))
    (:`then_1`
      (add `Button.OnClicked` (`/Game/Widgets/WBP_StoreWidget.TakeButton` _aswbp_store_widget) (delegate `TakeItem`)))))

(event `TakeItem`
  (bind (_storeditemstack_item _storeditemstack_itemquantity) (break `/Game/GameManage/ST_ItemStack` (`self.StoredItemStack`)))
  (bind _storeditemstack (`self.StoredItemStack`))
  (`KismetSystemLibrary.PrintText` (`KismetTextLibrary.Conv_StringToText` (`KismetStringLibrary.Concat_StrStr` (`KismetStringLibrary.Conv_NameToString` (break `/Game/GameManage/ST_Item` (break `/Game/GameManage/ST_ItemStack` _storeditemstack))) "" (`KismetStringLibrary.Conv_IntToString` (`.ItemID_10_05E1392B4735FFE91395E096C0362B11` (break `/Game/GameManage/ST_Item` (break `/Game/GameManage/ST_ItemStack` _storeditemstack)))) "" (`KismetSystemLibrary.GetDisplayName` (`.Sprite_12_C3E3BEF7482375E8B6ED59A9B46A7A49` (break `/Game/GameManage/ST_Item` (break `/Game/GameManage/ST_ItemStack` _storeditemstack)))) "" (`KismetStringLibrary.Conv_IntToString` (`.DisplayCode_14_DA320A0F46F774CC85313AB0D355DB03` (break `/Game/GameManage/ST_Item` (break `/Game/GameManage/ST_ItemStack` _storeditemstack)))) "" (`KismetStringLibrary.Conv_DoubleToString` (`.ItemCost_20_EF3CC9BC4D8F1FE198FCE58B55A35F26` (break `/Game/GameManage/ST_Item` (break `/Game/GameManage/ST_ItemStack` _storeditemstack)))) "" (`KismetStringLibrary.Conv_IntToString` (`.ItemQuantity_4_F5DAE9484DE62FBE49B5F0A69999838A` (break `/Game/GameManage/ST_ItemStack` _storeditemstack))))))
  (if (!= _storeditemstack_itemquantity 0)
    (bind _returnvalue (`|SpawnActorFromClass` "/Game/Storage/BP_StoredItem.BP_StoredItem_C" (`SceneComponent.K2_GetComponentToWorld` (`self.SpawnPoint`)) "AlwaysSpawn" "MultiplyWithRoot" null null null))
    (set `/Game/Storage/BP_StoredItem.ItemInfo` (`self.StoredItemStack`) _returnvalue)
    (set `/Game/Storage/BP_StoredItem.BaseDepthX` -4100.0 _returnvalue)
    (set `self.StoredItemStack` (make `/Game/GameManage/ST_ItemStack` (struct)))
    (else
      (`KismetSystemLibrary.PrintText` "Nothing here"))))

(event `self.SlotCollision.OnComponentBeginOverlap`
  (params (OverlappedComponent :type "PrimitiveComponent Object Reference") (OtherActor :type "Actor Object Reference") (OtherComp :type "PrimitiveComponent Object Reference") (OtherBodyIndex :type Integer) (bFromSweep :type Boolean) (SweepResult :type "HitResult Structure (by ref)"))
  (bind (_storeditemstack_item _storeditemstack_itemquantity) (break `/Game/GameManage/ST_ItemStack` (`self.StoredItemStack`)))
  (bind _newparam (message `/Game/BP_Main/BPI_Storable.Store Preview` OtherActor (== _storeditemstack_itemquantity 0) null))
  (set `self.Potential Item` _newparam))

(event `self.SlotCollision.OnComponentEndOverlap`
  (params (OverlappedComponent :type "PrimitiveComponent Object Reference") (OtherActor :type "Actor Object Reference") (OtherComp :type "PrimitiveComponent Object Reference") (OtherBodyIndex :type Integer))
  (message `/Game/BP_Main/BPI_Storable.StorePreviewStop` OtherActor))

(event `Add potential item`
  (bind _potential_item (`self.Potential Item`))
  (bind _potential_item_item (break `/Game/GameManage/ST_ItemStack` (`self.Potential Item`)))
  (bind (_item _itemquantity) (break `/Game/GameManage/ST_ItemStack` (`self.StoredItemStack`)))
  (if (== (`.ItemID_10_05E1392B4735FFE91395E096C0362B11` (break `/Game/GameManage/ST_Item` _item)) (`.ItemID_10_05E1392B4735FFE91395E096C0362B11` (break `/Game/GameManage/ST_Item` (break `/Game/GameManage/ST_ItemStack` _potential_item)))) :!label _label
    (set `self.StoredItemStack` (make `/Game/GameManage/ST_ItemStack` _potential_item_item (+ _itemquantity (`.ItemQuantity_4_F5DAE9484DE62FBE49B5F0A69999838A` (break `/Game/GameManage/ST_ItemStack` _potential_item)))))
    (else
      (if (not (== _itemquantity 0))
        (bind _returnvalue (`|SpawnActorFromClass` "/Game/Storage/BP_StoredItem.BP_StoredItem_C" (`SceneComponent.K2_GetComponentToWorld` (`self.SpawnPoint`)) "AlwaysSpawn" "MultiplyWithRoot" null null null))
        (set `/Game/Storage/BP_StoredItem.ItemInfo` (`self.StoredItemStack`) _returnvalue)
        (set `/Game/Storage/BP_StoredItem.BaseDepthX` -4100.0 _returnvalue))
      (set `self.StoredItemStack` (`self.Potential Item`))
      (cast `/Game/BP_Main/BuildShopGameState` (`GameplayStatics.GetGameState`)))))

(event `AddItem`
  (params (ItemToAdd :type "/Game/GameManage/ST_ItemStack Structure"))
  (set `self.Potential Item` ItemToAdd)
  (goto _label))

(fn `UserConstructionScript`)