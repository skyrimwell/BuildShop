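; Storage base Blueprint that previews and accepts items placed into a storage slot.
; When an item enters, it asks the item for a store preview, passing whether the last stored stack is empty, and keeps the result as the potential item.
; Leaving stops that preview.
; Adding either the potential item or a given item fires OnAddItem, which is empty here.
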(event `OnItemEnter`
  (params (Item :type "Actor Object Reference"))
  (bind (_laststoreditemstack_item _laststoreditemstack_itemquantity) (break `/Game/GameManage/ST_ItemStack` (`self.LastStoredItemStack`)))
  (bind _newparam (message `/Game/BP_Main/BPI_Storable.Store Preview` Item (== _laststoreditemstack_itemquantity 0) self))
  (set `self.Potential Item` _newparam))

(event `OnItemOut`
  (params (Item :type "Actor Object Reference"))
  (message `/Game/BP_Main/BPI_Storable.StorePreviewStop` Item))

(event `Add potential item`
  (`self.OnAddItem` (`self.Potential Item`) :!label _label))

(event `AddItem`
  (params (ItemToAdd :type "/Game/GameManage/ST_ItemStack Structure"))
  (set `self.Potential Item` ItemToAdd)
  (goto _label))

(event `OnAddItem`
  (params (Item :type "/Game/GameManage/ST_ItemStack Structure")))

(fn `UserConstructionScript`)