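; Draggable physics item for shop storage that displays its item's mesh and can be dropped into a storage slot.
; Clicking grabs it by center of mass with a PhysicsHandle; while not AtTheStorage, Tick projects the cursor onto a fixed world-Y plane read from a data table.
; Slot preview calls track overlaps and the target slot.
; On release it either notifies the slot and destroys itself, or returns to its ReturnPoint after a delay.
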(event `/Game/BP_Main/BPI_Clickable1.OnObjectClicked`
  (bind _returnvalue (`GameplayStatics.GetPlayerController` 0))
  (bind _iteminfo (`self.ItemInfo`))
  (bind (_bblockinghit _binitialoverlap _time _distance _location _impactpoint _normal _impactnormal _physmat _hitactor _hitcomponent) (`GameplayStatics.BreakHitResult` (`PlayerController.GetHitResultUnderCursorByChannel` _returnvalue "TraceTypeQuery1" true)))
  (`/Game/BP_Main/BP_DraggableComponent.OnParentClicked` (`self.BP_DraggableComponent`))
  (bind _asbp_shop_pawn (cast `/Game/BP_Main/BP_ShopPawn` (`GameplayStatics.GetPlayerPawn` 0)))
  (set `self.At the Storage` (`/Game/BP_Main/BP_ShopPawn.AtTheStorage` _asbp_shop_pawn))
  (`PrimitiveComponent.SetEnableGravity` (`self.SM`) false)
  (set `self.GoOffDragging` false)
  (`KismetSystemLibrary.PrintString` (`KismetStringLibrary.Concat_StrStr` (`KismetStringLibrary.Conv_NameToString` (break `/Game/GameManage/ST_Item` (break `/Game/GameManage/ST_ItemStack` _iteminfo))) " \n" (`KismetStringLibrary.Conv_IntToString` (`.ItemID_10_05E1392B4735FFE91395E096C0362B11` (break `/Game/GameManage/ST_Item` (break `/Game/GameManage/ST_ItemStack` _iteminfo)))) " \n" (`KismetStringLibrary.Conv_IntToString` (`.ItemQuantity_4_F5DAE9484DE62FBE49B5F0A69999838A` (break `/Game/GameManage/ST_ItemStack` _iteminfo)))))
  (set `self.PC_Ref` _returnvalue)
  (if (== (`ActorComponent.GetOwner` _hitcomponent) self)
    (`PhysicsHandleComponent.GrabComponentAtLocation` (`self.PhysicsHandle`) (`self.SM`) "None" (`PrimitiveComponent.GetCenterOfMass` _hitcomponent "None"))
    (set `self.isDragging` true)
    (else
      (`PrimitiveComponent.SetEnableGravity` (`self.SM`) true)
      (`self.OnObjectReleased` false))))

(event `self.ReceiveTick`
  (params (DeltaSeconds :type "Float (single-precision)"))
  (bind _pc_ref (`self.PC_Ref`))
  (bind (_locationx _locationy) (`PlayerController.GetMousePosition` _pc_ref))
  (bind (_worldposition _worlddirection) (`GameplayStatics.DeprojectScreenToWorld` _pc_ref (`KismetMathLibrary.MakeVector2D` _locationx _locationy)))
  (if (`self.isDragging`)
    (if (not (`self.At the Storage`))
      (`PhysicsHandleComponent.SetTargetLocation` (`self.PhysicsHandle`) (+ _worldposition (* _worlddirection (`KismetMathLibrary.SafeDivide` (- (`self.BaseDepthX`) (.y _worldposition)) (.y _worlddirection)))))
      ;[1 1 1] Выход из стейта захвата
      (if (`self.GoOffDragging`)
        (set `self.GoOffDragging` false)
        (`PhysicsHandleComponent.ReleaseComponent` (`self.PhysicsHandle`))
        (set `self.isDragging` false)
        (if (`self.TargetBoxSelected`)
          (`/Game/BP_Main/BPI_Storable.Store`)
          (else
            ;[1 1 1] Гашение инерции
            (`PhysicsHandleComponent.SetTargetLocation` (`self.PhysicsHandle`) (`SceneComponent.RelativeLocation` (`self.SM`)))
            (`KismetSystemLibrary.Delay` 0.5)
            (`self.ReturnToPoint`)))))))

(event `self.ReceiveBeginPlay`
  (bind _bp_draggablecomponent (`self.BP_DraggableComponent`))
  (bind (_itemname _itemid _sprite _displaycode _itemcost _mesh) (break `/Game/GameManage/ST_Item` (`.Item_5_E57DE2F4450938253A738EB3F08E417F` (break `/Game/GameManage/ST_ItemStack` (`self.ItemInfo`)))))
  (`StaticMeshComponent.SetStaticMesh` (`self.SM`) _mesh)
  (`KismetSystemLibrary.PrintString` (`KismetStringLibrary.Concat_StrStr` "I set new static mesh: " (`KismetSystemLibrary.GetObjectName` _mesh)))
  (set `self.PC_Ref` (`GameplayStatics.GetPlayerController` 0))
  (bind _returnvalue (`|GetDataTableRow` "/Game/GameManage/DT_GlobalVariables.DT_GlobalVariables" "BaseDepthStorage")
    (:`then`
      (set `self.BaseDepthX` (break `/Game/GameManage/ST_GlobalVariables` _returnvalue))
      (set `/Game/BP_Main/BP_DraggableComponent.SM` (`self.SM`) _bp_draggablecomponent)
      (set `/Game/BP_Main/BP_DraggableComponent.Physics Handle` (`self.PhysicsHandle`) _bp_draggablecomponent))))

(event `/Game/BP_Main/BPI_Clickable1.OnObjectReleased`
  (params (IsHolded :type Boolean))
  (set `self.GoOffDragging` true)
  (`PrimitiveComponent.SetEnableGravity` (`self.SM`) true))

(event `/Game/BP_Main/BPI_Storable.StorePreviewStop`
  (bind _returnvalue (- (`self.OverlappingCount`) 1))
  (if (== _returnvalue -1)
    (set `self.OverlappingCount` 0)
    (set `self.TargetBoxSelected` false :!label _label)
    (set `self.SlotRef` null)
    (else
      (bind _output_get (set `self.OverlappingCount` _returnvalue))
      (if (== _output_get 0)
        (goto _label)))))

(event `/Game/BP_Main/BPI_Storable.Store`
  (bind _sm (`self.SM`))
  (`/Engine/EditorBlueprintResources/StandardMacros.IsValid` (`self.SlotRef`)
    (:`Is Valid`
      (`/Game/Storage/BP_StorageBase.Add potential item` (`self.SlotRef`)))
    (:`Is Not Valid`
      _))
  (`PrimitiveComponent.SetEnableGravity` _sm false)
  (`PrimitiveComponent.SetSimulatePhysics` _sm false)
  (`/Engine/EditorBlueprintResources/StandardMacros.IsValid` self
    (:`Is Valid`
      (`self.K2_DestroyActor` self))))

(fn `GetInfo`
  (returns (NewParam1 :type "/Game/GameManage/ST_ItemStack Structure"))
  (set `self.TargetBoxSelected` true)
  (return (`self.ItemInfo`)))

(fn `Initialization`
  (params (Item :type "/Game/GameManage/ST_ItemStack Structure"))
  (bind (_itemname _itemid _sprite _displaycode _itemcost _mesh) (break `/Game/GameManage/ST_Item` (`.Item_5_E57DE2F4450938253A738EB3F08E417F` (break `/Game/GameManage/ST_ItemStack` (`self.ItemInfo`)))))
  (`KismetSystemLibrary.PrintString` (`KismetSystemLibrary.GetObjectName` _mesh))
  (set `self.ItemInfo` Item)
  (`StaticMeshComponent.SetStaticMesh` (`self.SM`) _mesh))

(fn `ReturnToPoint`
  (bind _returnpoint (`self.ReturnPoint`))
  (bind _sm (`self.SM`))
  (`/Engine/EditorBlueprintResources/StandardMacros.IsValid` _returnpoint
    (:`Is Valid`
      (`KismetSystemLibrary.PrintString` "ValidPoint")
      (`PrimitiveComponent.SetSimulatePhysics` _sm true)
      (`SceneComponent.K2_SetRelativeLocation` _sm (`self.K2_GetActorLocation` _returnpoint) false false))
    (:`Is Not Valid`
      (`KismetSystemLibrary.PrintString` "PointIsNotValid"))))

(fn `Store Preview`
  (params (IsFree :type Boolean) (StorageSlot :type "/Game/Storage/BP_StorageBase Object Reference"))
  (returns (NewParam :type "/Game/GameManage/ST_ItemStack Structure"))
  (set `self.SlotRef` StorageSlot)
  (set `self.TargetBoxSelected` true)
  (bind _result (`/Engine/EditorBlueprintResources/StandardMacros.IncrementInt` (`self.OverlappingCount`))
    (:`  `
      (set `self.OverlappingCount` _result)
      (return (`self.ItemInfo`)))))

(fn `UserConstructionScript`)