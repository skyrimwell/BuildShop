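; Test static shop cart that collects storable items and checks them against the game state's current order.
; Box overlap reads item info through BPI_Storable into StoredItems; a whole-struct match inserts a summed entry rather than replacing the existing one.
; ApplyOrder prints OrderCompare's result, which compares array lengths, then ID and quantity, though only the last ordered item's match decides.
; Debug prints trace additions; end overlap does nothing.
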(event `self.Box.OnComponentBeginOverlap`
  (params (OverlappedComponent :type "PrimitiveComponent Object Reference") (OtherActor :type "Actor Object Reference") (OtherComp :type "PrimitiveComponent Object Reference") (OtherBodyIndex :type Integer) (bFromSweep :type Boolean) (SweepResult :type "HitResult Structure (by ref)"))
  (if (`KismetSystemLibrary.DoesImplementInterface` OtherActor "/Game/BP_Main/BPI_Storable.BPI_Storable_C")
    (bind _newparam1 (message `/Game/BP_Main/BPI_Storable.GetInfo` OtherActor))
    (`self.AddItemToCart` _newparam1)))

(event `ApplyOrder`
  (bind _asbuild_shop_game_state (cast `/Game/BP_Main/BuildShopGameState` (`GameplayStatics.GetGameState`)))
  (bind (_isequal _whatwrong) (`self.OrderCompare` (`/Game/BP_Main/BuildShopGameState.CurrentOrder` _asbuild_shop_game_state) (`self.StoredItems`)))
  (`KismetSystemLibrary.PrintString` _whatwrong)
  (if _isequal
    _))

(event `self.Box.OnComponentEndOverlap`
  (params (OverlappedComponent :type "PrimitiveComponent Object Reference") (OtherActor :type "Actor Object Reference") (OtherComp :type "PrimitiveComponent Object Reference") (OtherBodyIndex :type Integer)))

(fn `AddItemToCart`
  (params (ItemInput :type "/Game/GameManage/ST_ItemStack Structure"))
  (bind (_item _itemquantity) (break `/Game/GameManage/ST_ItemStack` ItemInput))
  (bind _returnvalue (`KismetArrayLibrary.Array_Find` (`self.StoredItems`) ItemInput))
  (bind (_output_item _output_itemquantity) (break `/Game/GameManage/ST_ItemStack` (`|GetArrayItem` (`self.StoredItems`) _returnvalue)))
  (bind (_item_2 _itemquantity_2) (break `/Game/GameManage/ST_ItemStack` (`|GetArrayItem` (`self.StoredItems`) _returnvalue)))
  (if (>= _returnvalue 0)
    ;[1 1 1] Если айтем уже в корзине, суммируем
    (`KismetArrayLibrary.Array_Insert` (`self.StoredItems`) (make `/Game/GameManage/ST_ItemStack` _item (+ _itemquantity _output_itemquantity)) _returnvalue)
    (`KismetSystemLibrary.PrintString` (`KismetStringLibrary.Concat_StrStr` (`KismetStringLibrary.Conv_NameToString` (break `/Game/GameManage/ST_Item` _item_2)) "-----" (`KismetStringLibrary.Conv_IntToString` _itemquantity_2) "Если айтем уже в корзине, суммируем") true true (struct :`R` 0.083815 :`G` 1.0 :`B` 0.018095 :`A` 1.0) 10.0)
    (else
      ;[1 1 1] Если айтем не в корзине, добавляем
      (`KismetArrayLibrary.Array_Add` (`self.StoredItems`) (make `/Game/GameManage/ST_ItemStack` _item _itemquantity))
      (`KismetSystemLibrary.PrintString` (`KismetStringLibrary.Concat_StrStr` (`KismetStringLibrary.Conv_NameToString` (`.ItemName_17_324A2A684139DC36CE4A499CA48A2CAB` (break `/Game/GameManage/ST_Item` _item))) "------" (`KismetStringLibrary.Conv_IntToString` _itemquantity) "Если айтем не в корзине, добавляем") true true (struct :`G` 1.0 :`B` 0.053283 :`A` 1.0) 10.0))))

(fn `OrderCompare`
  (params (GeneratedOrder :type "/Game/GameManage/ST_CustomerOrder Structure") (StoredItems :type "Array of /Game/GameManage/ST_ItemStack Structure"))
  (returns (IsEqual :type Boolean) (WhatWrong :type String))
  (locals (bFoundMatch :type Boolean) (LGeneratedOrder :type "Array of /Game/GameManage/ST_ItemStack Structure") (LStoredItems :type "Array of /Game/GameManage/ST_ItemStack Structure"))
  (set `local.LGeneratedOrder` GeneratedOrder_Items_19_92E324BF40B28E2E42823A94930C01BA)
  (set `local.LStoredItems` StoredItems)
  (if (== (`KismetArrayLibrary.Array_Length` (`local.LGeneratedOrder`)) (`KismetArrayLibrary.Array_Length` (`local.LStoredItems`)))
    ;[1 1 1] Сравнение по содержимому
    (for _array_element (`local.LGeneratedOrder`)
      (set `local.bFoundMatch` false)
      (for _array_element_2 (`local.LStoredItems`)
        (if (and (== (`.ItemID_10_05E1392B4735FFE91395E096C0362B11` (break `/Game/GameManage/ST_Item` (break `/Game/GameManage/ST_ItemStack` _array_element_2))) (`.ItemID_10_05E1392B4735FFE91395E096C0362B11` (break `/Game/GameManage/ST_Item` (break `/Game/GameManage/ST_ItemStack` _array_element)))) (== (`.ItemQuantity_4_F5DAE9484DE62FBE49B5F0A69999838A` (break `/Game/GameManage/ST_ItemStack` _array_element_2)) (`.ItemQuantity_4_F5DAE9484DE62FBE49B5F0A69999838A` (break `/Game/GameManage/ST_ItemStack` _array_element))))
          (set `local.bFoundMatch` true))))
    (if (`local.bFoundMatch`)
      (return true "Все норм")
      (else
        (return false "Что-то не соответствует")))
    (else
      (return false "Different size"))))

(fn `UserConstructionScript`)