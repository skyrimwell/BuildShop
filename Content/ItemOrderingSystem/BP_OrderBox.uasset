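; BP_OrderBox is an order box actor in the item ordering system that stores the items passed to it.
; AddItems takes a map of items and appends each value to StoredItems, discarding the keys.
; It then prints the name, ID and cost of every stored item, apparently as debug output.
; The box has no other active logic.
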(event `AddItems`
  (params (ItemsToAdd :type "Map of Integer to /Game/GameManage/ST_ItemStack Structure"))
  (bind _keys (`BlueprintMapLibrary.Map_Keys` ItemsToAdd))
  (for _array_element _keys
    (`KismetArrayLibrary.Array_Add` (`self.StoredItems`) (`BlueprintMapLibrary.Map_Find` ItemsToAdd _array_element)))
  (for _array_element_2 (`self.StoredItems`)
    (bind (_itemname _itemid _sprite _displaycode _itemcost) (break `/Game/GameManage/ST_Item` (break `/Game/GameManage/ST_ItemStack` _array_element_2)))
    (`KismetSystemLibrary.PrintString` (`KismetStringLibrary.Concat_StrStr` (`KismetStringLibrary.Conv_NameToString` _itemname) " \n \n" (`KismetStringLibrary.Conv_IntToString` _itemid) " \n \n" (`KismetStringLibrary.Conv_DoubleToString` _itemcost)))))

(fn `UserConstructionScript`)