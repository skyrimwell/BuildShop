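; BP_OrderManager generates random customer orders for the shop, each pairing a dialogue line with a list of item stacks.
; GenOrder picks a dialogue row (skipping the first), then draws the requested number of random items and quantities from data tables.
; MakeOrder stores the order in BuildShopGameState, then GenOrder adds each item to its map under indexed "SH_" slot names.
; TestOrder is a debug event; CreateNewOrder is empty.
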(event `MakeOrder`
  (params (SelectedLine :type "/Game/GameManage/ST_Dialogues Structure") (SelectedItems :type "Array of /Game/GameManage/ST_ItemStack Structure"))
  ;[1 1 1] Собрать заказ
  (set `self.CurrentOrder` (make `/Game/GameManage/ST_CustomerOrder` SelectedLine SelectedItems))
  ;[1 1 1] Установка текущего заказа в GameState
  (bind _asbuild_shop_game_state (cast `/Game/BP_Main/BuildShopGameState` (`GameplayStatics.GetGameState`)))
  (`/Game/BP_Main/BuildShopGameState.SetCurrentOrder` _asbuild_shop_game_state (`self.CurrentOrder`)))

(event `GenOrder`
  (params (Amount :type Integer))
  (bind _dialoguerownames (`self.DialogueRowNames`))
  (bind _generateditems (`self.GeneratedItems`))
  ;[1 1 1] Получаем доступные предметы и диалоги
  (bind _outrownames (`DataTableFunctionLibrary.GetDataTableRowNames` (`self.DialogueDataTable`)))
  (set `self.DialogueRowNames` _outrownames)
  (bind _outrownames_2 (`DataTableFunctionLibrary.GetDataTableRowNames` (`self.ItemDataTable`)))
  (set `self.ItemRowNames` _outrownames_2)
  ;[1 1 1] Вытаскиваем случайную реплику
  (bind _returnvalue (`|GetDataTableRow` (`self.DialogueDataTable`) (`|GetArrayItem` _dialoguerownames (`KismetMathLibrary.RandomIntegerInRange` 1 (- (`KismetArrayLibrary.Array_Length` _dialoguerownames) 1))))
    (:`then`
      (bind (_lineid _line) (break `/Game/GameManage/ST_Dialogues` _returnvalue))
      (set `self.SelectedDialogue` (make `/Game/GameManage/ST_Dialogues` _lineid _line))
      ;[1 1 1] Ген предметов в заказе
      (bind _output_get (set `self.ItemsToGenerate` (- Amount 1)))
      (for _ (range (+ _output_get 1))
        (bind _returnvalue_2 (`|GetDataTableRow` (`self.ItemDataTable`) (`|GetArrayItem` (`self.ItemRowNames`) (`KismetMathLibrary.RandomIntegerInRange` 0 (- (`KismetArrayLibrary.Array_Length` (`self.ItemRowNames`)) 1))))
          (:`then`
            (bind (_itemname _itemid _sprite _displaycode _itemcost _mesh) (break `/Game/GameManage/ST_Item` _returnvalue_2))
            (bind (_st_itemstack_item _st_itemstack_itemquantity) (break `/Game/GameManage/ST_ItemStack` (make `/Game/GameManage/ST_ItemStack` (make `/Game/GameManage/ST_Item` _itemname _itemid _sprite _displaycode _itemcost _mesh) (`KismetMathLibrary.RandomIntegerInRange` 1 30))))
            (`KismetArrayLibrary.Array_Add` (`self.GeneratedItems`) (make `/Game/GameManage/ST_ItemStack` _st_itemstack_item _st_itemstack_itemquantity)))))
      (`self.MakeOrder` (`self.SelectedDialogue`) _generateditems)
      (bind _asbuild_shop_game_state (cast `/Game/BP_Main/BuildShopGameState` (`GameplayStatics.GetGameState`)))
      (for (_array_element _array_index) _generateditems
        (`/Game/BP_Main/BuildShopGameState.Add Item To Map` _asbuild_shop_game_state _array_element (`KismetStringLibrary.Conv_StringToName` (`KismetStringLibrary.Concat_StrStr` "SH_" (`KismetStringLibrary.Conv_IntToString` _array_index))))))
    (:`RowNotFound`
      (`KismetSystemLibrary.PrintString` "Пизда диалог проебало"))))

(event `TestOrder`
  (bind (_currentorder_customerline _currentorder_items) (break `/Game/GameManage/ST_CustomerOrder` (`self.CurrentOrder`)))
  ;[1 1 1] Отладка
  (`self.GenOrder` 0)
  (`KismetSystemLibrary.PrintString` "///Тест создания///")
  (`KismetSystemLibrary.PrintString` (`KismetStringLibrary.Concat_StrStr` "Клиент пиздит: " (`KismetTextLibrary.Conv_TextToString` (`.Line_5_A716A56D4096CFFCCFD39D9F4EA8DC51` (break `/Game/GameManage/ST_Dialogues` (`.CustomerLine_17_9CF2553F47B2FF21E8DF58A2F9E7782F` (break `/Game/GameManage/ST_CustomerOrder` (`self.CurrentOrder`))))))))
  (`KismetSystemLibrary.PrintString` "В заказе следующие товары: " true true (struct :`G` 0.66 :`B` 1.0 :`A` 1.0) 5.0)
  (for _array_element _currentorder_items
    (`KismetSystemLibrary.PrintText` (`KismetTextLibrary.Conv_StringToText` (`KismetStringLibrary.Concat_StrStr` "" " \n" "" " \n" "" " \n" "" " \n" "" " \n" "/////Айтем сгенерен/////")) true true (struct :`G` 0.66 :`B` 1.0 :`A` 1.0) 7.0))
  (`KismetSystemLibrary.PrintString` "///Отладка все гг///" true true (struct :`G` 0.66 :`B` 1.0 :`A` 1.0) 7.0))

(fn `CreateNewOrder`)

(fn `UserConstructionScript`)