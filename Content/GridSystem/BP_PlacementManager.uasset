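; Placement manager that lets the player place, pick back up and rotate decor objects in the shop.
; Each tick it projects the cursor onto a floor plane and sphere-overlaps for free BP_DecorPoints, easing the preview actor into the snap transform.
; On release, the point accepts the preview or placement cancels and destroys it.
; Placed objects report pickup and selection through dispatchers, while WBP_SelectInterface and ShopPlayerController events drive rotation.
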(event `self.ReceiveTick`
  (params (DeltaSeconds :type "Float (single-precision)"))
  (bind _previewactorref (`self.PreviewActorRef`))
  (bind _pcref (`self.PCRef`))
  (bind (_locationx _locationy) (`PlayerController.GetMousePosition` _pcref))
  (bind (_worldposition _worlddirection) (`GameplayStatics.DeprojectScreenToWorld` _pcref (`KismetMathLibrary.MakeVector2D` _locationx _locationy)))
  (bind (_t _intersection) (`KismetMathLibrary.LinePlaneIntersection_OriginNormal` _worldposition (+ _worldposition (* _worlddirection 100000.0)) (`KismetMathLibrary.MakeVector` 0.0 0.0 (`self.FloorZ`)) (0.0 0.0 1.0)))
  (if (`self.IsPlacing`)
    (`/Engine/EditorBlueprintResources/StandardMacros.IsValid` (`self.PreviewActorRef`)
      (:`Is Valid`
        (if (not (`self.IsSnapping`))
          (`self.K2_SetActorLocation` (`self.PreviewActorRef`) _intersection false false))
        (bind (_outactors _returnvalue) (`KismetSystemLibrary.SphereOverlapActors` _intersection (`self.SnapEnterRadius`) (`|MakeArray` (`self.ObjType`)) "/Game/GridSystem/PointVersion/BP_DecorPoint.BP_DecorPoint_C"))
        (if _returnvalue
          (set `self.minDistance` 99999.0)
          (for _array_element _outactors
            (bind _asbp_decor_point (cast `/Game/GridSystem/PointVersion/BP_DecorPoint` _array_element))
            (if (`KismetSystemLibrary.IsValid` _asbp_decor_point)
              (if (not (`/Game/GridSystem/PointVersion/BP_DecorPoint.bOccupied` _asbp_decor_point))
                (bind _mounttransform (`/Game/GridSystem/PointVersion/BP_DecorPoint.getSnapTransform` _asbp_decor_point))
                (bind _location (.location _mounttransform))
                (if (< (`KismetMathLibrary.VSize` (- _location _intersection)) (`self.minDistance`))
                  (set `self.bestPoint` _asbp_decor_point)
                  (set `self.bestSnapLocation` _location)
                  (set `self.BestSnapRotation` (.rotation _mounttransform))))))
          (if (`KismetSystemLibrary.IsValid` (`self.bestPoint`))
            (set `self.IsSnapping` true)
            (`self.K2_SetActorLocation` (`self.PreviewActorRef`) (`KismetMathLibrary.VInterpTo` (`self.K2_GetActorLocation` _previewactorref) (`self.bestSnapLocation`) DeltaSeconds 3.0) false false)
            (`self.K2_SetActorRotation` (`self.PreviewActorRef`) (`KismetMathLibrary.RInterpTo` (`self.K2_GetActorRotation` _previewactorref) (`self.BestSnapRotation`) DeltaSeconds 3.0) false)
            (set `/Game/GridSystem/BP_DecorObjectPreview.bSnapped` true (`self.PreviewActorRef`))
            (set `self.CurrentSnapPoint` (`self.bestPoint`))
            (else
              (set `self.IsSnapping` true)
              (set `/Game/GridSystem/BP_DecorObjectPreview.bSnapped` false (`self.PreviewActorRef`))
              (`self.K2_SetActorLocation` (`KismetMathLibrary.VInterpTo` (`self.K2_GetActorLocation` (`self.PreviewActorRef`)) _intersection DeltaSeconds 3.0))))
          (else
            (set `self.IsSnapping` false)))))))

(event `TakeItem`
  (params (ObjectReference :type "/Game/GridSystem/BP_DecorObjectPreview Object Reference"))
  ;[1 1 1] Взяли предмет
  (`Widget.RemoveFromParent` (`self.SelectWidget`))
  (remove `/Game/GridSystem/BP_DecorObjectPreview.ItemHasTaked` ObjectReference (delegate `TakeItem`))
  (set `self.IsPlacing` true)
  (set `self.PreviewActorRef` ObjectReference)
  (bind _asshop_player_controller (cast `/Game/BP_Main/ShopPlayerController` (`GameplayStatics.GetPlayerController` 0)))
  (set `/Game/BP_Main/ShopPlayerController.LastClickedActor` self _asshop_player_controller)
  (set `/Game/BP_Main/ShopPlayerController.bClickedPending` true _asshop_player_controller)
  (set `self.PreviewActorRef` ObjectReference))

(event `/Game/BP_Main/BPI_Clickable1.OnObjectReleased`
  (params (IsHolded :type Boolean))
  (if (`self.IsSnapping`)
    (`self.ConfirmPlacement`)
    (else
      (`self.CancelPlacement`))))

(event `self.ReceiveDestroyed`
  (`Widget.RemoveFromParent` (`self.SelectWidget`)))

(event `ConnectDispatcher`
  (bind _previewactorref (`self.PreviewActorRef`))
  ;[1 1 1] Установка диспатчера для каждого preview Actor
  (add `/Game/GridSystem/BP_DecorObjectPreview.ItemHasTaked` _previewactorref (delegate `TakeItem`))
  (add `/Game/GridSystem/BP_DecorObjectPreview.NewActiveObject` _previewactorref (delegate `SelectNewActiveObject`)))

(event `SelectNewActiveObject`
  (params (ActiveObjectReference :type "/Game/GridSystem/BP_DecorObjectPreview Object Reference"))
  (bind _selectwidget (`self.SelectWidget`))
  (bind (_origin _boxextent) (`self.GetActorBounds` (`self.ActiveActor`) false false))
  (bind (_x _y) (`KismetMathLibrary.BreakVector2D` (`GameplayStatics.ProjectWorldToScreen` (`GameplayStatics.GetPlayerController` 0) (- _origin (/ _boxextent 2.0)))))
  (if (`self.PlacingMode`)
    (set `self.ActiveActor` ActiveObjectReference)
    (`/Engine/EditorBlueprintResources/StandardMacros.IsValid` (`self.SelectWidget`)
      (:`Is Valid`
        _)
      (:`Is Not Valid`
        (bind _returnvalue (`|CreateWidget` "/Game/GridSystem/WBP_SelectInterface.WBP_SelectInterface_C" (`GameplayStatics.GetPlayerController` 0)))
        (bind _output_get (set `self.SelectWidget` _returnvalue))
        (add `/Game/GridSystem/WBP_SelectInterface.StartRotation` _output_get (delegate `StartRotationObject`))
        (add `/Game/GridSystem/WBP_SelectInterface.StopRotation` _output_get (delegate `StopRotationObject`))))
    (if (not (`Widget.IsInViewport` _selectwidget))
      (`UserWidget.AddToViewport` _selectwidget 0))
    (`KismetSystemLibrary.DelayUntilNextTick`)
    (`UserWidget.SetPositionInViewport` (`self.SelectWidget`) (`KismetMathLibrary.MakeVector2D` (- _x (/ (`SizeBox.WidthOverride` (`/Game/GridSystem/WBP_SelectInterface.SizeBox_100` (`self.SelectWidget`))) 2.0)) _y) true)
    (`UserWidget.SetPositionInViewport` _returnvalue (`KismetMathLibrary.MakeVector2D` (- _x (/ (`SizeBox.WidthOverride` (`/Game/GridSystem/WBP_SelectInterface.SizeBox_100` (`self.SelectWidget`))) 2.0)) _y) true)))

(event `self.ReceiveBeginPlay`
  ;[1 1 1] Comment
  (bind _asshop_player_controller (cast `/Game/BP_Main/ShopPlayerController` (`GameplayStatics.GetPlayerController` 0)))
  (add `/Game/BP_Main/ShopPlayerController.RotationEvent` _asshop_player_controller (delegate `StartRotationObject`))
  (add `/Game/BP_Main/ShopPlayerController.StopRotationEvent` _asshop_player_controller (delegate `StopRotationObject`)))

(event `CancelSelectAction`
  (bind _selectwidget (`self.SelectWidget`))
  (set `self.PlacingMode` false)
  (set `self.ActiveActor` null)
  (`/Engine/EditorBlueprintResources/StandardMacros.IsValid` _selectwidget
    (:`Is Valid`
      (`Widget.RemoveFromParent` _selectwidget))))

(event `StartRotationObject`
  (params (IsRightRotation :type Boolean))
  (bind _activeactor (`self.ActiveActor`))
  ;[1 1 1] StartRotation
  (`/Engine/EditorBlueprintResources/StandardMacros.IsValid` _activeactor
    (:`Is Valid`
      (`/Game/GridSystem/BP_DecorObjectPreview.StartRotation` _activeactor IsRightRotation))))

(event `StopRotationObject`
  (bind _activeactor (`self.ActiveActor`))
  ;[1 1 1] StopRotation
  (`/Engine/EditorBlueprintResources/StandardMacros.IsValid` _activeactor
    (:`Is Valid`
      (`/Game/GridSystem/BP_DecorObjectPreview.StopRotation` _activeactor))))

(fn `CancelPlacement`
  (bind _previewactorref (`self.PreviewActorRef`))
  (`/Engine/EditorBlueprintResources/StandardMacros.IsValid` _previewactorref
    (:`Is Valid`
      (`self.K2_DestroyActor` _previewactorref)
      (set `self.PreviewActorRef` null)
      (set `self.CurrentSnapPoint` null)
      (set `self.IsPlacing` false)
      (`self.PlacementFinish` false))))

(fn `ConfirmPlacement`
  (bind _previewactorref (`self.PreviewActorRef`))
  (`/Engine/EditorBlueprintResources/StandardMacros.IsValid` _previewactorref
    (:`Is Valid`
      (if (and (`/Game/GridSystem/BP_DecorObjectPreview.bSnapped` _previewactorref) (`KismetSystemLibrary.IsValid` (`self.CurrentSnapPoint`)))
        (bind _isaccepted (`/Game/GridSystem/PointVersion/BP_DecorPoint.AcceptItem` (`self.CurrentSnapPoint`) (`self.PreviewActorRef`)))
        (if _isaccepted
          (set `self.IsPlacing` false)
          (`self.K2_SetActorLocation` (`self.PreviewActorRef`) (`self.K2_GetActorLocation` (`self.CurrentSnapPoint`)) false false)
          (`self.ConnectDispatcher`)
          (set `self.PreviewActorRef` null)
          (set `self.CurrentSnapPoint` null)
          (`self.PlacementFinish` true)
          (else
            (`self.CancelPlacement`)))))))

(fn `StartPlacement`
  (params (ItemData :type "/Game/GridSystem/ST_PlacementObject Structure") (PC :type "PlayerController Object Reference"))
  (bind _output_get (set `self.CurrentItemData` ItemData))
  (set `self.PCRef` PC)
  (bind _returnvalue (`|SpawnActorFromClass` "/Game/GridSystem/BP_DecorObjectPreview.BP_DecorObjectPreview_C" (`KismetMathLibrary.MakeTransform` (0.0 0.0 0.0)) "Undefined" "MultiplyWithRoot" null _output_get null))
  (set `self.PreviewActorRef` _returnvalue)
  (set `self.IsPlacing` true)
  (bind _asshop_player_controller (cast `/Game/BP_Main/ShopPlayerController` (`GameplayStatics.GetPlayerController` 0)))
  (set `/Game/BP_Main/ShopPlayerController.LastClickedActor` self _asshop_player_controller)
  (set `/Game/BP_Main/ShopPlayerController.bClickedPending` true _asshop_player_controller))

(fn `UserConstructionScript`)