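; BP_DecorPoint is a placement point in the point-based grid system that holds one decor item.
; On BeginPlay it moves its decor object, billboard and mount to a wall or floor offset based on IsWallObject.
; GetSnapTransform exposes the mount's world transform for snapping.
; AcceptItem stores an item and marks the point occupied only if it is free and the item's allowed point type matches, printing a debug message on mismatch.
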(event `self.ReceiveBeginPlay`
  (bind _decorobject (`self.DecorObject`))
  (bind _wallpos (`self.WallPos`))
  (bind _floorpos (`self.FloorPos`))
  (bind _billboard (`self.Billboard`))
  (if (`self.isWallObject`)
    (`SceneComponent.K2_SetRelativeLocation` _decorobject _wallpos false false)
    (`SceneComponent.K2_SetRelativeLocation` _billboard _wallpos false false)
    (`SceneComponent.K2_SetRelativeLocation` (`self.Mount`) _wallpos false false)
    (else
      (`SceneComponent.K2_SetRelativeLocation` _decorobject _floorpos false false)
      (`SceneComponent.K2_SetRelativeLocation` _billboard _floorpos false false)
      (`SceneComponent.K2_SetRelativeLocation` (`self.Mount`) _floorpos false false))))

(fn `AcceptItem`
  (params (ItemData :type "/Game/GridSystem/BP_DecorObjectPreview Object Reference"))
  (returns (IsAccepted :type Boolean))
  (if (`self.bOccupied`)
    (return false)
    (elif (`|EnumEquality` (`self.ObjectTypes`) (`.AllowedPointType_21_02AB417F42553D6253FF5FB51D530340` (break `/Game/GridSystem/ST_PlacementObject` (`/Game/GridSystem/BP_DecorObjectPreview.ItemData` ItemData))))
      (set `self.Occupant` ItemData)
      (set `self.bOccupied` true)
      (return true)
      (else
        (`KismetSystemLibrary.PrintString` "Ты проебался с enum")
        (return false)))))

(fn `getSnapTransform`
  (returns (MountTransform :type "Transform Structure"))
  (return (`SceneComponent.K2_GetComponentToWorld` (`self.Mount`))))

(fn `UserConstructionScript`)