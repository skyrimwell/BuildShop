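; BP_InstancedGridObject is a clickable object in the grid system, identified by a two-component InstanceIndex.
; On click, it prints its X,Y coordinates and calls the OnObjectBeingCalled dispatcher with that index.
; Release and Box hit events only print debug text, while the Box's own click event and the construction script are empty.
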(event `/Game/BP_Main/BPI_Clickable1.OnObjectClicked`
  (bind (_instanceindex_x _instanceindex_y) (break `IntPoint` (`self.instanceIndex`)))
  (`KismetSystemLibrary.PrintString` (`KismetStringLibrary.Concat_StrStr` "(" (`KismetStringLibrary.Conv_IntToString` _instanceindex_x) "," (`KismetStringLibrary.Conv_IntToString` _instanceindex_y) ")"))
  (`self.OnObjectBeingCalled` (`self.instanceIndex`)))

(event `self.Box.OnComponentHit`
  (params (HitComponent :type "PrimitiveComponent Object Reference") (OtherActor :type "Actor Object Reference") (OtherComp :type "PrimitiveComponent Object Reference") (NormalImpulse :type "Vector Structure") (Hit :type "HitResult Structure (by ref)"))
  (`KismetSystemLibrary.PrintString` "Hit"))

(event `self.Box.OnClicked`
  (params (TouchedComponent :type "PrimitiveComponent Object Reference") (ButtonPressed :type "Key Structure")))

(event `/Game/BP_Main/BPI_Clickable1.OnObjectReleased`
  (params (IsHolded :type Boolean))
  (`KismetSystemLibrary.PrintString` "releas"))

(fn `UserConstructionScript`)