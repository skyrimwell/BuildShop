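; BP_DecorObjectPreview is a placeable decor item actor for shop decoration, showing the static mesh from its item data.
; A hold in decoration state signals that the item was taken, while a non-held release signals it as the new active object.
; Start and stop events toggle Tick-driven yaw rotation in either direction, at a speed read from the global variables DataTable.
; Preview mode is only stored, and validity feedback is an empty stub.
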(event `self.ReceiveBeginPlay`
  (bind _returnvalue (`|GetDataTableRow` "/Game/GameManage/DT_GlobalVariables.DT_GlobalVariables" "DesignRotationSpeed")
    (:`then`
      (set `self.RotationSpeed` (break `/Game/GameManage/ST_GlobalVariables` _returnvalue)))
    (:`RowNotFound`
      _))
  (`StaticMeshComponent.SetStaticMesh` (`self.SM_Preview`) (`.mesh_14_47FD027340BDA68AD7631EB847044880` (break `/Game/GridSystem/ST_PlacementObject` (`self.ItemData`)))))

(event `/Game/BP_Main/BPI_Clickable1.OnObjectHolded`
  (`KismetSystemLibrary.PrintString` "Hello")
  (bind _asshop_player_controller (cast `/Game/BP_Main/ShopPlayerController` (`GameplayStatics.GetPlayerController` 0)))
  (if (`/Game/BP_Main/ShopPlayerController.DecorationState` _asshop_player_controller)
    (`self.ItemHasTaked` self)))

(event `/Game/BP_Main/BPI_Clickable1.OnObjectClicked`)

(event `/Game/BP_Main/BPI_Clickable1.OnObjectReleased`
  (params (IsHolded :type Boolean))
  (if (not IsHolded)
    (`self.NewActiveObject` self)))

(event `StartRotation`
  (params (IsRightRotation :type Boolean))
  (set `self.IsRightRotation` IsRightRotation)
  (set `self.RotatingNow` true)
  (`KismetSystemLibrary.PrintString` "I'm enabled again"))

(event `StopRotation`
  (set `self.RotatingNow` false)
  (`KismetSystemLibrary.PrintString` "I'm set rotating now in false"))

(event `self.ReceiveTick`
  (params (DeltaSeconds :type "Float (single-precision)"))
  (bind _roll (.roll (`self.K2_GetActorRotation`)))
  (bind _pitch (.pitch (`self.K2_GetActorRotation`)))
  (bind _yaw (.yaw (`self.K2_GetActorRotation`)))
  (bind _returnvalue (* DeltaSeconds (`self.RotationSpeed`)))
  (if (`self.RotatingNow`)
    (if (`self.IsRightRotation`)
      (`self.K2_SetActorRotation` (`KismetMathLibrary.MakeRotator` _roll _pitch (- _yaw _returnvalue)))
      (else
        (`self.K2_SetActorRotation` (`KismetMathLibrary.MakeRotator` _roll _pitch (+ _yaw _returnvalue)))))))

(fn `SetItemData`
  (params (ItemData :type "/Game/GridSystem/ST_PlacementObject Structure"))
  (set `self.ItemData` ItemData)
  (`StaticMeshComponent.SetStaticMesh` (`self.SM_Preview`) (`.mesh_14_47FD027340BDA68AD7631EB847044880` (break `/Game/GridSystem/ST_PlacementObject` ItemData))))

(fn `SetPreviewMode`
  (params (`isPreview?` :type Boolean))
  (set `self.bIsPreview` `isPreview?`))

(fn `SetValidPreview`
  (params (Valid :type Boolean)))

(fn `UserConstructionScript`)