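; BP_GridBase is a grid actor that builds a flat, rectangular grid of cells at runtime on BeginPlay.
; It clears the Cells array, then loops over GridWidth and GridHeight, storing each cell's XY position as a CellSize step offset by GridRoot's world location.
; Each cell also gets an InstancedStaticMesh instance scaled to CellSize, added in local space despite that world-location offset.
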(event `self.ReceiveBeginPlay`
  (bind _cellsize (`self.CellSize`))
  (bind (_returnvalue_x _returnvalue_y) (`KismetMathLibrary.BreakVector` (`SceneComponent.K2_GetComponentLocation` (`self.GridRoot`))))
  (bind _returnvalue (/ (`self.CellSize`) 100.0))
  (`KismetArrayLibrary.Array_Clear` (`self.Cells`))
  (for _index (range (`self.GridWidth`))
    (for _index_2 (range (`self.GridHeight`))
      (bind _returnvalue_2 (+ (`KismetMathLibrary.MakeVector2D` (* _index _cellsize) (* _index_2 _cellsize)) (`KismetMathLibrary.MakeVector2D` _returnvalue_x _returnvalue_y)))
      (`KismetArrayLibrary.Array_Add` (`self.Cells`) _returnvalue_2)
      (bind (_x _y) (`KismetMathLibrary.BreakVector2D` _returnvalue_2))
      (`InstancedStaticMeshComponent.AddInstance` (`self.InstancedStaticMesh`) (`KismetMathLibrary.MakeTransform` (`KismetMathLibrary.MakeVector` _x _y) (struct) (`KismetMathLibrary.MakeVector` _returnvalue _returnvalue 0.5)) false))))

(fn `UserConstructionScript`)