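; Placement manager that lets the player position decor item previews with the cursor and snap them to BP_DecorPoint actors.
; StartPlacement spawns a preview for new items, then Tick cursor-traces and sphere-overlaps to pick the nearest type-matching point with a valid Occupant.
; ConfirmPlacement attaches the preview, sets it as Occupant and opens WBP_DecorPanel; CancelPlacement destroys it unless PreviousPoint is valid.
; Re-placing existing items and ShowPointsForTypes are unfinished stubs.
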(event `self.ReceiveBeginPlay`
  (bind _outactors (`GameplayStatics.GetAllActorsOfClass` "/Game/GridSystem/PointVersion/BP_DecorPoint.BP_DecorPoint_C"))
  (set `self.DecorPoints` _outactors))

(event `self.ReceiveTick`
  (params (DeltaSeconds :type "Float (single-precision)"))
  (bind _bestpoint (`self.BestPoint`))
  (bind _currentpreview (`self.CurrentPreview`))
  (bind (_currentitemdata_id _currentitemdata_name _currentitemdata_cost _currentitemdata_mesh _currentitemdata_icon _currentitemdata_tooltip _currentitemdata_allowedpointtype) (break `/Game/GridSystem/ST_PlacementObject` (`self.CurrentItemData`)))
  (bind _hitresult (`PlayerController.GetHitResultUnderCursorByChannel` (`GameplayStatics.GetPlayerController` 0) (`self.PlacementTraceChannel`) true))
  (if (`self.bIsPlacing`)
    (`/Engine/EditorBlueprintResources/StandardMacros.IsValid` (`self.CurrentPreview`)
      (:`Is Valid`
        (`self.K2_SetActorLocation` (`self.CurrentPreview`) (`.TraceStart` (`GameplayStatics.BreakHitResult` _hitresult)) false false)
        (bind _outactors (`KismetSystemLibrary.SphereOverlapActors` (`.TraceStart` (`GameplayStatics.BreakHitResult` _hitresult)) (`self.SnapRadius`) (`|MakeArray` (`self.ObjectTypeQuery`)) "/Game/GridSystem/PointVersion/BP_DecorPoint.BP_DecorPoint_C"))
        (for _array_element _outactors
          (bind _asbp_decor_point (cast `/Game/GridSystem/PointVersion/BP_DecorPoint` _array_element)
            (:`then`
              _)
            (:`CastFailed`
              _))
          (if (and (`|EnumEquality` _currentitemdata_allowedpointtype (`/Game/GridSystem/PointVersion/BP_DecorPoint.ObjectTypes` _asbp_decor_point)) (`KismetSystemLibrary.IsValid` (`/Game/GridSystem/PointVersion/BP_DecorPoint.Occupant` _asbp_decor_point)))
            (bind _returnvalue (`KismetMathLibrary.Vector_Distance` (`SceneComponent.K2_GetComponentLocation` (`/Game/GridSystem/PointVersion/BP_DecorPoint.Mount` _asbp_decor_point)) (`.Location` (`GameplayStatics.BreakHitResult` _hitresult))))
            (if (< _returnvalue (`self.BestDist`))
              (set `self.BestDist` _returnvalue)
              (set `self.BestPoint` _asbp_decor_point))))
        (if (`KismetSystemLibrary.IsValid` (`self.BestPoint`))
          (set `self.SnappedPoint` _bestpoint)
          (bind _mounttransform (`/Game/GridSystem/PointVersion/BP_DecorPoint.getSnapTransform` _bestpoint))
          (`self.K2_SetActorTransform` _currentpreview _mounttransform false false)
          (`/Game/GridSystem/BP_DecorObjectPreview.SetValidPreview` _currentpreview true)
          (else
            (set `self.SnappedPoint` null)
            (`/Game/GridSystem/BP_DecorObjectPreview.SetValidPreview` (`self.CurrentPreview`) true)))))))

(fn `CancelPlacement`
  (if (`KismetSystemLibrary.IsValid` (`self.PreviousPoint`))
    (return)
    (else
      (`self.K2_DestroyActor` (`self.CurrentPreview`))
      (set `self.bIsPlacing` false))))

(fn `ConfirmPlacement`
  (bind _snappedpoint (`self.SnappedPoint`))
  (bind _currentpreview (`self.CurrentPreview`))
  (`/Engine/EditorBlueprintResources/StandardMacros.IsValid` (`self.SnappedPoint`)
    (:`Is Valid`
      (`self.K2_AttachToActor` _currentpreview _snappedpoint "None" "KeepRelative" "KeepRelative" "KeepRelative" true)
      (set `/Game/GridSystem/PointVersion/BP_DecorPoint.Occupant` _currentpreview _snappedpoint)
      (bind _returnvalue (`|CreateWidget` "/Game/GridSystem/newVersion/WBP_DecorPanel.WBP_DecorPanel_C"))
      (`UserWidget.AddToViewport` _returnvalue 0))))

(fn `ShowPointsForTypes`
  (params (Types :type Boolean) (bShow :type Boolean))
  (for _array_element (`self.DecorPoints`)
    (bind _asbp_decor_point (cast `/Game/GridSystem/PointVersion/BP_DecorPoint` _array_element))
    (if (and (`/Game/GridSystem/PointVersion/BP_DecorPoint.isWallObject` _asbp_decor_point) Types)
      _)))

(fn `StartPlacement`
  (params (ItemData :type "/Game/GridSystem/ST_PlacementObject Structure") (bWasPlacedBefore :type Boolean))
  (bind (_hitresult _returnvalue) (`PlayerController.GetHitResultUnderCursorByChannel` (`GameplayStatics.GetPlayerController` 0) (`self.PlacementTraceChannel`) true))
  (set `self.CurrentItemData` ItemData)
  (if (not bWasPlacedBefore)
    (set `self.PreviousPoint` null)
    (if _returnvalue
      (bind _returnvalue_2 (`|SpawnActorFromClass` "/Game/GridSystem/BP_DecorObjectPreview.BP_DecorObjectPreview_C" (`KismetMathLibrary.MakeTransform` (`.Location` (`GameplayStatics.BreakHitResult` _hitresult))) "Undefined" "MultiplyWithRoot" null null))
      (`/Game/GridSystem/BP_DecorObjectPreview.SetItemData` _returnvalue_2 (`self.CurrentItemData`))
      (`/Game/GridSystem/BP_DecorObjectPreview.SetPreviewMode` _returnvalue_2 true)
      (set `self.CurrentPreview` _returnvalue_2)
      (set `self.bIsPlacing` true))))

(fn `UserConstructionScript`
  (set `self.DecorPointQueryRadius` (* (`self.SnapRadius`) 1.2)))